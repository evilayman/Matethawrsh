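; Button actor in the safety object spawning system that asks a SpawnerManager to spawn its SafetyObject.
; Both actor overlap and a Tick-driven three-second Delay trigger the spawn, so it also fires without contact.
; A CoolDown flag blocks repeat spawns until CoolDownTime elapses, then the spawned object returns to the manager's unused list.
; The motion controller cast is disconnected, so overlaps are not filtered by actor type.
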(event `self.ReceiveActorBeginOverlap`
  (params (OtherActor :type "Actor Object Reference"))
  (if (not (`self.coolDown`)) :!label _label
    (bind _spawnedsafetyobject (`/Game/Project/Blueprints/SpawningSafetyObjectSystem/SpawnManager.SpawnObject` (`self.spawnerManager`) (`self.safetyObject`)))
    (set `self.coolDown` true)
    (`KismetSystemLibrary.Delay` (`self.coolDownTime`))
    (set `self.coolDown` false)
    (`/Game/Project/Blueprints/SpawningSafetyObjectSystem/SpawnManager.ReturnSafetyObjectToUnusedList` (`self.spawnerManager`) _spawnedsafetyobject)))

(event `self.ReceiveTick`
  (params (DeltaSeconds :type "Float (single-precision)"))
  (`KismetSystemLibrary.Delay` 3.0)
  (goto _label))

(fn `UserConstructionScript`)