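; Actor component that records its owner's movement and plays it backwards to rewind the object.
; While recording, Tick stores transform, linear and angular physics velocities and step durations in Record, capping repeated identical samples at MaxRedundantMoves.
; StartRewind thins the record and stops recording, then Tick pops and applies samples newest-first, delayed by stored durations rather than the computed OneStepRewindTime.
; An emptied record triggers StopRewind, which fires the completion dispatcher.
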(event `self.ReceiveBeginPlay`)

(event `self.ReceiveTick`
  (params (DeltaSeconds :type "Float (single-precision)"))
  (if (`self.RewindStarted`)
    (if (< (`KismetArrayLibrary.Array_LastIndex` (`.Transforms_3_920AE801440DC98B056C4D9D987D380F` (break `/Game/Project/Blueprints/BP_Rewind/RecordData` (`self.Record`)))) 0)
      (`self.StopRewind`)
      (else
        (`self.RewindOneStep` (`self.OneStepRewindTime`))))
    (elif (`self.RecordStarted`)
      (`self.RecordMovement`))))

(event `self.StartRecording`
  (params (MaxRedundantMoves :type Integer) (Record :type "/Game/Project/Blueprints/BP_Rewind/RecordData Structure (by ref)"))
  (set `self.Record` Record)
  (`self.StopRecording`)
  (`self.StopRewind`)
  (set `self.MaxRedundantMoves` MaxRedundantMoves)
  (set `self.RecordStarted` true))

(event `self.StopRecording`
  (set `self.RecordStarted` false))

(event `self.StartRewind`
  (params (Time :type "Float (single-precision)"))
  (bind _returnvalue (`KismetArrayLibrary.Array_Length` (`.Transforms_3_920AE801440DC98B056C4D9D987D380F` (break `/Game/Project/Blueprints/BP_Rewind/RecordData` (`self.Record`)))))
  (`self.SkipRecord` 1)
  (if (> _returnvalue 0)
    (`self.StopRecording`)
    (if (not (`self.RewindStarted`))
      (set `self.RewindStarted` true)
      (set `self.OneStepRewindTime` (/ Time (`KismetMathLibrary.Conv_IntToDouble` _returnvalue))))))

(event `self.StopRewind`
  (bind (_transforms _linearvels _angularvels _bonedata _stepdurations) (break `/Game/Project/Blueprints/BP_Rewind/RecordData` (`self.Record`)))
  (if (`self.RewindStarted`)
    (`self.Disp_RewindCompleted`))
  (set `self.RewindStarted` false)
  (set `self.IsRewinding` false)
  (`KismetArrayLibrary.Array_Clear` _transforms)
  (`KismetArrayLibrary.Array_Clear` _linearvels)
  (`KismetArrayLibrary.Array_Clear` _angularvels)
  (set `self.RedundantMovesCounter` 0)
  (`KismetArrayLibrary.Array_Clear` _stepdurations))

(fn `RecordMovement`
  (locals (StepTime :type "Float (double-precision)"))
  (bind _returnvalue (`self.GetOwner`))
  (bind _returnvalue_2 (`self.GetOwner`))
  (bind (_transforms _linearvels _angularvels _bonedata _stepdurations) (break `/Game/Project/Blueprints/BP_Rewind/RecordData` (`self.Record`)))
  (bind _transforms_2 (break `/Game/Project/Blueprints/BP_Rewind/RecordData` (`self.Record`)))
  (bind (_transforms_3 _linearvels_2 _angularvels_2) (break `/Game/Project/Blueprints/BP_Rewind/RecordData` (`self.Record`)))
  (bind _returnvalue_3 (`Actor.GetComponentByClass` _returnvalue "/Script/Engine.PrimitiveComponent"))
  (bind _returnvalue_4 (`Actor.GetComponentByClass` _returnvalue_2 "/Script/Engine.PrimitiveComponent"))
  (bind _returnvalue_5 (`PrimitiveComponent.GetPhysicsAngularVelocityInDegrees` _returnvalue_4 "None"))
  (set `local.StepTime` (`.PartialSeconds` (`GameplayStatics.GetAccurateRealTime`)))
  (if (> (`KismetArrayLibrary.Array_Length` _transforms) 0)
    (`|ExecutionSequence`
      (:`then_0`
        (if (== (`|GetArrayItem` _transforms_2 (`KismetArrayLibrary.Array_LastIndex` _transforms_2)) (`Actor.GetTransform` _returnvalue_2))
          (bind _result (`/Engine/EditorBlueprintResources/StandardMacros.IncrementInt` (`self.RedundantMovesCounter`))
            (:`  `
              (if (not (>= _result (`self.MaxRedundantMoves`)))
                (`KismetArrayLibrary.Array_Add` _transforms_2 (`Actor.GetTransform` _returnvalue_2) :!label _label))))
          (else
            (set `self.RedundantMovesCounter` 0)
            (goto _label))))
      (:`then_1`
        (bind _returnvalue_6 (`PrimitiveComponent.GetPhysicsLinearVelocity` _returnvalue_4 "None"))
        (if (== (`|GetArrayItem` _linearvels_2 (`KismetArrayLibrary.Array_LastIndex` _linearvels_2)) _returnvalue_6)
          (if (not (>= (`self.RedundantMovesCounter`) (`self.MaxRedundantMoves`)))
            (`KismetArrayLibrary.Array_Add` _linearvels_2 _returnvalue_6 :!label _label_2))
          (else
            (goto _label_2))))
      (:`then_2`
        (if (== (`|GetArrayItem` _angularvels_2 (`KismetArrayLibrary.Array_LastIndex` _angularvels_2)) _returnvalue_5)
          (if (not (>= (`self.RedundantMovesCounter`) (`self.MaxRedundantMoves`)))
            (`KismetArrayLibrary.Array_Add` _angularvels_2 _returnvalue_5 :!label _label_3))
          (else
            (goto _label_3))))
      (:`then_3`
        (bind _output_get (set `local.StepTime` (- (`.PartialSeconds` (`GameplayStatics.GetAccurateRealTime`)) (`local.StepTime`))))
        (`KismetArrayLibrary.Array_Add` (`.StepDurations_12_9278CDB94170104F3786E6BC343F7247` (break `/Game/Project/Blueprints/BP_Rewind/RecordData` (`self.Record`))) _output_get)))
    (else
      (`KismetArrayLibrary.Array_Add` _transforms (`Actor.GetTransform` _returnvalue))
      (bind _returnvalue_7 (`PrimitiveComponent.GetPhysicsLinearVelocity` _returnvalue_3 "None"))
      (`KismetArrayLibrary.Array_Add` _linearvels _returnvalue_7)
      (`KismetArrayLibrary.Array_Add` _angularvels (`PrimitiveComponent.GetPhysicsAngularVelocityInDegrees` _returnvalue_3 "None"))
      (`KismetArrayLibrary.Array_Add` _stepdurations))))

(fn `SkipRecord`
  (params (SkipRate :type Integer))
  (bind (_transforms _linearvels _angularvels _bonedata _stepdurations) (break `/Game/Project/Blueprints/BP_Rewind/RecordData` (`self.Record`)))
  (if (!= SkipRate 0)
    (for _index (range (+ (`KismetArrayLibrary.Array_Length` (`.Transforms_3_920AE801440DC98B056C4D9D987D380F` (break `/Game/Project/Blueprints/BP_Rewind/RecordData` (`self.Record`)))) 1))
      (if (== (mod _index 1) 0)
        (`KismetArrayLibrary.Array_Remove` _transforms _index)
        (`KismetArrayLibrary.Array_Remove` _linearvels _index)
        (`KismetArrayLibrary.Array_Remove` _angularvels _index)
        (`KismetArrayLibrary.Array_Remove` _bonedata _index)
        (`KismetArrayLibrary.Array_Remove` _stepdurations _index)))))