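; MC_Accident5_2 is a path point for a rewindable character that stages an accident depending on whether a hole is safe.
; On arrival it applies its active state and marks work done, then branches on the MC's IsHoleSafe flag.
; A safe hole resets the state and moves the character on after timed delays, while an unsafe one summons the Shinigami after a pause.
; Arrival during rewind moves the character straight on.
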(event `self.OnPointArrive`
  (params (RewindableCharacter :type "/Game/Project/Blueprints/BP_Rewind/BP_RewindableCharacter Object Reference"))
  (`parent.OnPointArrive` RewindableCharacter)
  (`self.SetActiveState` (`self.ActiveState`))
  (`self.SetWorkDone` true)
  (if (`/Game/Project/MainCharacter/BP_MC.IsHoleSafe` (`self.MC`))
    (`KismetSystemLibrary.Delay` 4.0)
    (`self.SetActiveState` 0)
    (`KismetSystemLibrary.Delay` 1.0)
    (`self.MoveOn` 150.0)
    (else
      (`KismetSystemLibrary.Delay` 2.0)
      (`self.SummonShinigami` "NewEnumerator6"))))

(event `self.OnPointArriveRewind`
  (params (`Rewindable Character` :type "/Game/Project/Blueprints/BP_Rewind/BP_RewindableCharacter Object Reference"))
  (`parent.OnPointArriveRewind` `Rewindable Character`)
  (`self.MoveOn` 150.0))

(fn `UserConstructionScript`
  (`parent.UserConstructionScript`))