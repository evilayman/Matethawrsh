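; VR table with three buttons that spawn safety objects, beneath animated glove, eyewear and hat displays.
; A timeline hovers and spins the displays from BeginPlay.
; Overlapping a button sphere sets its cooldown and red material before the motion controller cast, then depresses it and requests its object from SpawnerManager.
; After CoolDownTime, the button resets and the object returns to the manager's unused pool.
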(event `self.ReceiveBeginPlay`
  (bind _floatingglove (`self.FloatingGlove`))
  ;[1 1 1] Object Rotation and Hover
  (bind (_direction _rotatordelta _hovervector) (`Timeline|HoverandRotator`)
    (:`Update`
      (`|ExecutionSequence`
        (:`then_0`
          (`SceneComponent.K2_AddLocalOffset` _floatingglove _hovervector false false)
          (`SceneComponent.K2_AddLocalOffset` (`self.FloatingEyewear`) _hovervector false false)
          (`SceneComponent.K2_AddLocalOffset` (`self.FloatingHat`) _hovervector false false))
        (:`then_1`
          (`SceneComponent.K2_SetRelativeRotation` _floatingglove (`KismetMathLibrary.MakeRotator` 0.0 0.0 _rotatordelta) false false)
          (`SceneComponent.K2_SetRelativeRotation` (`self.FloatingEyewear`) (`KismetMathLibrary.MakeRotator` 0.0 0.0 _rotatordelta) false false)
          (`SceneComponent.K2_SetRelativeRotation` (`self.FloatingHat`) (`KismetMathLibrary.MakeRotator` 0.0 0.0 _rotatordelta) false false))))))

(event `self.Sphere01.OnComponentBeginOverlap`
  (params (OverlappedComponent :type "PrimitiveComponent Object Reference") (OtherActor :type "Actor Object Reference") (OtherComp :type "PrimitiveComponent Object Reference") (OtherBodyIndex :type Integer) (bFromSweep :type Boolean) (SweepResult :type "HitResult Structure (by ref)"))
  ;[1 1 1] Buttons Overlap Logic
  (if (not (`self.CoolDownB1`))
    (set `self.CoolDownB1` true)
    (`PrimitiveComponent.SetMaterial` (`self.Button01`) 0 "/Game/Alaa/M_Red.M_Red")
    (cast `/Game/VirtualRealityBP/Blueprints/BP_MotionController` OtherActor)
    (`|ExecutionSequence`
      (:`then_0`
        (`self.Movement1` (`self.Button01`)))
      (:`then_1`
        (`self.SpawnObject1` (`|GetArrayItem` (`self.SafetyObject`)))))))

(event `self.Sphere02.OnComponentBeginOverlap`
  (params (OverlappedComponent :type "PrimitiveComponent Object Reference") (OtherActor :type "Actor Object Reference") (OtherComp :type "PrimitiveComponent Object Reference") (OtherBodyIndex :type Integer) (bFromSweep :type Boolean) (SweepResult :type "HitResult Structure (by ref)"))
  ;[1 1 1] Buttons Overlap Logic
  (if (not (`self.CoolDownB2`))
    (set `self.CoolDownB2` true)
    (`PrimitiveComponent.SetMaterial` (`self.Button02`) 0 "/Game/Alaa/M_Red.M_Red")
    (cast `/Game/VirtualRealityBP/Blueprints/BP_MotionController` OtherActor)
    (`|ExecutionSequence`
      (:`then_0`
        (`self.Movement2` (`self.Button02`)))
      (:`then_1`
        (`self.SpawnObject2` (`|GetArrayItem` (`self.SafetyObject`) 1))))))

(event `self.Sphere03.OnComponentBeginOverlap`
  (params (OverlappedComponent :type "PrimitiveComponent Object Reference") (OtherActor :type "Actor Object Reference") (OtherComp :type "PrimitiveComponent Object Reference") (OtherBodyIndex :type Integer) (bFromSweep :type Boolean) (SweepResult :type "HitResult Structure (by ref)"))
  ;[1 1 1] Buttons Overlap Logic
  (if (not (`self.CoolDownB3`))
    (set `self.CoolDownB3` true)
    (`PrimitiveComponent.SetMaterial` (`self.Button03`) 0 "/Game/Alaa/M_Red.M_Red")
    (cast `/Game/VirtualRealityBP/Blueprints/BP_MotionController` OtherActor)
    (`|ExecutionSequence`
      (:`then_0`
        (`self.Movement3` (`self.Button03`)))
      (:`then_1`
        (`self.SpawnObject3` (`|GetArrayItem` (`self.SafetyObject`) 2))))))

(event `Movement1`
  (params (Button_Sekeletal_Mesh_Component :type "SkeletalMeshComponent Object Reference"))
  ;[1 1 1] Buttons Overlap Logic
  (`SceneComponent.K2_AddLocalOffset` Button_Sekeletal_Mesh_Component (0.0 0.0 -2.0) false true)
  (`KismetSystemLibrary.Delay` (`self.CoolDownTime`))
  (`SceneComponent.K2_AddLocalOffset` Button_Sekeletal_Mesh_Component (0.0 0.0 2.0) false true)
  (`PrimitiveComponent.SetMaterial` Button_Sekeletal_Mesh_Component 0 "/Game/Alaa/M_Green.M_Green"))

(event `Movement2`
  (params (Button_Sekeletal_Mesh_Component :type "SkeletalMeshComponent Object Reference"))
  ;[1 1 1] Buttons Overlap Logic
  (`SceneComponent.K2_AddLocalOffset` Button_Sekeletal_Mesh_Component (0.0 0.0 -2.0) false true)
  (`KismetSystemLibrary.Delay` (`self.CoolDownTime`))
  (`SceneComponent.K2_AddLocalOffset` Button_Sekeletal_Mesh_Component (0.0 0.0 2.0) false true)
  (`PrimitiveComponent.SetMaterial` Button_Sekeletal_Mesh_Component 0 "/Game/Alaa/M_Green.M_Green"))

(event `Movement3`
  (params (Button_Sekeletal_Mesh_Component :type "SkeletalMeshComponent Object Reference"))
  ;[1 1 1] Buttons Overlap Logic
  (`SceneComponent.K2_AddLocalOffset` Button_Sekeletal_Mesh_Component (0.0 0.0 -2.0) false true)
  (`KismetSystemLibrary.Delay` (`self.CoolDownTime`))
  (`SceneComponent.K2_AddLocalOffset` Button_Sekeletal_Mesh_Component (0.0 0.0 2.0) false true)
  (`PrimitiveComponent.SetMaterial` Button_Sekeletal_Mesh_Component 0 "/Game/Alaa/M_Green.M_Green"))

(event `SpawnObject1`
  (params (SafetyObject :type "/Game/Project/Blueprints/SafetyEquipments/NewSafetyObjects/BP_EndlessThrowable Class Reference"))
  ;[1 1 1] Buttons Overlap Logic
  (bind _spawnedsafetyobject (`/Game/Project/Blueprints/SpawningSafetyObjectSystem/SpawnManager.SpawnObject` (`self.SpawnerManager`) SafetyObject))
  (`KismetSystemLibrary.Delay` (`self.CoolDownTime`))
  (set `self.CoolDownB1` false)
  (`/Game/Project/Blueprints/SpawningSafetyObjectSystem/SpawnManager.ReturnSafetyObjectToUnusedList` (`self.SpawnerManager`) _spawnedsafetyobject)
  (`KismetSystemLibrary.PrintString` "Hello" true true (struct :`G` 1.0 :`B` 0.018708 :`A` 1.0)))

(event `SpawnObject2`
  (params (SafetyObject :type "/Game/Project/Blueprints/SafetyEquipments/NewSafetyObjects/BP_EndlessThrowable Class Reference"))
  ;[1 1 1] Buttons Overlap Logic
  (bind _spawnedsafetyobject (`/Game/Project/Blueprints/SpawningSafetyObjectSystem/SpawnManager.SpawnObject` (`self.SpawnerManager`) SafetyObject))
  (`KismetSystemLibrary.Delay` (`self.CoolDownTime`))
  (set `self.CoolDownB2` false)
  (`/Game/Project/Blueprints/SpawningSafetyObjectSystem/SpawnManager.ReturnSafetyObjectToUnusedList` (`self.SpawnerManager`) _spawnedsafetyobject)
  (`KismetSystemLibrary.PrintString` "Hello"))

(event `SpawnObject3`
  (params (SafetyObject :type "/Game/Project/Blueprints/SafetyEquipments/NewSafetyObjects/BP_EndlessThrowable Class Reference"))
  ;[1 1 1] Buttons Overlap Logic
  (bind _spawnedsafetyobject (`/Game/Project/Blueprints/SpawningSafetyObjectSystem/SpawnManager.SpawnObject` (`self.SpawnerManager`) SafetyObject))
  (`KismetSystemLibrary.Delay` (`self.CoolDownTime`))
  (set `self.CoolDownB3` false)
  (`/Game/Project/Blueprints/SpawningSafetyObjectSystem/SpawnManager.ReturnSafetyObjectToUnusedList` (`self.SpawnerManager`) _spawnedsafetyobject)
  (`KismetSystemLibrary.PrintString` "Hello" true true (struct :`R` 1.0 :`B` 0.142866 :`A` 1.0)))

(fn `UserConstructionScript`)