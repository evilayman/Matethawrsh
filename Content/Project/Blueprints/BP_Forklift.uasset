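; Forklift actor that travels toward waypoints in its Points array, starting on BeginPlay.
; The MoveForkLift timeline lerps from the current location toward the first point, then removes it and starts RotateForkLift to yaw toward the next.
; Rotation does not chain into another move; the MoveFork event calls Play on the move timeline again.
; An unconnected LookAt transform node is left unused.
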(event `self.ReceiveBeginPlay`
  (bind _points (`self.Points`))
  (bind (_direction _alpha) (`Timeline|MoveForkLift` :!label _label)
    (:`Update`
      (`self.K2_SetActorLocation` (`KismetMathLibrary.VLerp` (`self.K2_GetActorLocation`) (`|GetArrayItem` _points) _alpha)))
    (:`Finished`
      (`KismetArrayLibrary.Array_Remove` _points)
      (bind (_direction_2 _alpha_2) (`Timeline|RotateForkLift`)
        (:`Update`
          (bind (_returnvalue_roll _returnvalue_pitch _returnvalue_yaw) (`KismetMathLibrary.BreakRotator` (`KismetMathLibrary.RLerp` (`self.K2_GetActorRotation`) (`KismetMathLibrary.FindLookAtRotation` (`self.K2_GetActorLocation`) (`|GetArrayItem` (`self.Points`))) _alpha_2)))
          (`self.K2_SetActorRotation` (`KismetMathLibrary.MakeRotator` 0.0 0.0 _returnvalue_yaw)))))))

(event `MoveFork`
  (goto _label))

(fn `UserConstructionScript`)