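; Shinigami apparition that is summoned on an accident, pauses time, speaks the next voice line and then resumes time, calling game over after the sixth.
; A flip-flopped timeline moves it between a fixed height and the summon point while driving dynamic fade materials and post-process saturation, reversing shortly before a rewind ends.
; A TV-line material is added to all post-process volumes after each non-final line and removed when the rewind completes.
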(event `self.ReceiveBeginPlay`
  (bind _outactors (`GameplayStatics.GetAllActorsOfClass` "/Script/Engine.PostProcessVolume"))
  (set `self.AllPostProcessRef` _outactors)
  (`self.K2_SetActorLocation` (0.0 0.0 -1000.0))
  (`AIController.K2_SetFocus` (`AIBlueprintHelperLibrary.GetAIController` self) (`GameplayStatics.GetPlayerController` 0))
  (`KismetArrayLibrary.Array_Clear` (`self.M_Fade`))
  (for (_ _array_index) (`MeshComponent.GetMaterials` (`self.Mesh`))
    (bind _returnvalue (`PrimitiveComponent.CreateDynamicMaterialInstance` (`self.Mesh`) _array_index "/Game/Project/Blueprints/Rewind_Effect/FadeOut/Nightshade_MAT_Fade.Nightshade_MAT_Fade" "None"))
    (`KismetArrayLibrary.Array_Add` (`self.M_Fade`) _returnvalue)))

(event `OnSummon`
  (params (Accident :type "/Game/Project/Blueprints/Enum_Shinigami Enum" :default "NewEnumerator6") (SummonLocation :type "Vector Structure"))
  (bind _output_get (set `self.SummonLocation` SummonLocation))
  (set `self.SumonLocation_z` (`KismetMathLibrary.MakeVector` (.x _output_get) (.y _output_get) -190.0))
  (`self.SetFadeAmountValue` 0.0)
  (`self.K2_SetActorLocation` (`self.SumonLocation_z`))
  (`self.AppearEvent`))

(event `OnSummonComplete`
  (bind _timerewinder (`self.TimeRewinder`))
  (bind _sumonlocation_z (`self.SumonLocation_z`))
  (bind _voicelinenumber (`self.VoiceLineNumber`))
  (`/Game/Project/Blueprints/BP_Rewind/TimeRewinder.StopTImeEvent` _timerewinder)
  (`/Game/Project/Blueprints/BP_Rewind/TimeRewinder.StopRecord` _timerewinder)
  (switch `int` (`self.VoiceLineNumber`)
    (:`0`
      (`GameplayStatics.SpawnSoundAtLocation` "/Game/Project/Sounds/Shinigami_1_Intro_Cue.Shinigami_1_Intro_Cue" _sumonlocation_z (struct) 1.0 1.0 0.0 "/Game/Project/Sounds/VoiceAttenuation.VoiceAttenuation" null)
      (`self.DilatedDelay` 7.5
        (:`Out`
          _)))
    (:`1`
      (`GameplayStatics.SpawnSoundAtLocation` "/Game/Project/Sounds/Shinigami_2_ElSabr.Shinigami_2_ElSabr" _sumonlocation_z (struct) 1.0 1.0 0.0 "/Game/Project/Sounds/VoiceAttenuation.VoiceAttenuation" null)
      (`self.DilatedDelay` 3.0
        (:`Out`
          _)))
    (:`2`
      (`GameplayStatics.SpawnSoundAtLocation` "/Game/Project/Sounds/Shinigami_3_Sab3Lo3_atV1.Shinigami_3_Sab3Lo3_atV1" _sumonlocation_z (struct) 1.0 1.0 0.0 "/Game/Project/Sounds/VoiceAttenuation.VoiceAttenuation" null)
      (`self.DilatedDelay` 5.0
        (:`Out`
          _)))
    (:`3`
      (`GameplayStatics.SpawnSoundAtLocation` "/Game/Project/Sounds/Shinigami_4_Sa7Sa7.Shinigami_4_Sa7Sa7" _sumonlocation_z (struct) 1.0 1.0 0.0 "/Game/Project/Sounds/VoiceAttenuation.VoiceAttenuation" null)
      (`self.DilatedDelay` 4.5
        (:`Out`
          _)))
    (:`4`
      (`GameplayStatics.SpawnSoundAtLocation` "/Game/Project/Sounds/Shinigami_5_Anameshmas2ol.Shinigami_5_Anameshmas2ol" _sumonlocation_z (struct) 1.0 1.0 0.0 "/Game/Project/Sounds/VoiceAttenuation.VoiceAttenuation" null)
      (`self.DilatedDelay` 5.5
        (:`Out`
          _)))
    (:`5`
      (`GameplayStatics.SpawnSoundAtLocation` "/Game/Project/Sounds/Shinigami_GameOver_MafeshFaida.Shinigami_GameOver_MafeshFaida" _sumonlocation_z (struct) 1.0 1.0 0.0 "/Game/Project/Sounds/VoiceAttenuation.VoiceAttenuation" null)
      (`self.DilatedDelay` 3.5
        (:`Out`
          _))))
  (set `self.VoiceLineNumber` (+ 1 _voicelinenumber))
  (if (== _voicelinenumber 6)
    (`self.GameOver`)
    (else
      (`/Game/Project/Blueprints/BP_Rewind/TimeRewinder.ResumeTimeEvent` (`self.TimeRewinder`))
      (`self.SetPostProcessTvMat`))))

(event `OnRewindStarted`
  (params (TimeForRewind :type "Float (double-precision)"))
  (`KismetSystemLibrary.Delay` (- TimeForRewind 1.0))
  (`self.AppearEvent`))

(event `OnRewindComplete`
  (`self.RemovePostProcessTvMat`))

(event `AppearEvent`
  ;[1 1 1] FadeEvent
  (`/Engine/EditorBlueprintResources/StandardMacros.FlipFlop`
    (:`A`
      (set `self.IsReverse` false)
      (bind (_direction _fadealpha _saturationalpha) (`Timeline|UpdateFade` :!via `PlayFromStart` :!label _label)
        (:`Update`
          (`self.SetFadeAmountValue` (`KismetMathLibrary.Lerp` 1.0 0.0 _fadealpha))
          (`self.K2_SetActorLocation` (`KismetMathLibrary.VLerp` (`self.SummonLocation`) (`self.SumonLocation_z`) _fadealpha))
          (if (`self.IsReverse`)
            (`self.SetPostProcessSaturation` 1.0)
            (else
              (`self.SetPostProcessSaturation` _saturationalpha))))
        (:`Finished`
          (if (`self.IsReverse`)
            (`self.K2_SetActorLocation` (0.0 0.0 -1000.0))
            (else
              (`self.OnSummonComplete`))))))
    (:`B`
      (set `self.IsReverse` true)
      (goto _label :!via `ReverseFromEnd`))))

(fn `RemovePostProcessTvMat`
  (locals (Mats :type "Array of WeightedBlendable Structure"))
  (for _array_element (`self.AllPostProcessRef`)
    (bind _weightedblendables_array (break `WeightedBlendables` (break `PostProcessSettings` (`PostProcessVolume.Settings` _array_element))))
    (`KismetArrayLibrary.Array_Remove` _weightedblendables_array (- (`KismetArrayLibrary.Array_Length` _weightedblendables_array) 1))
    (bind _weightedblendables_array_2 (break `WeightedBlendables` (break `PostProcessSettings` (`PostProcessVolume.Settings` _array_element))))
    (setmembers `PostProcessSettings` :`StructRef` (`PostProcessVolume.Settings` _array_element) :`WeightedBlendables` (make `WeightedBlendables` _weightedblendables_array_2))))

(fn `SetFadeAmountValue`
  (params (Value :type "Float (double-precision)"))
  (for _array_element (`self.M_Fade`)
    (`MaterialInstanceDynamic.SetScalarParameterValue` _array_element "FadeAmount" Value)))

(fn `SetPostProcessSaturation`
  (params (Alpha :type "Float (double-precision)"))
  (for _array_element (`self.AllPostProcessRef`)
    (setmembers `PostProcessSettings` :`StructRef` (`PostProcessVolume.Settings` _array_element) :`ColorSaturation` (`KismetMathLibrary.MakeVector4` 1.0 1.0 1.0 Alpha))))

(fn `SetPostProcessTvMat`
  (locals (Mats :type "Array of WeightedBlendable Structure"))
  (for _array_element (`self.AllPostProcessRef`)
    (bind _weightedblendables_array (break `WeightedBlendables` (break `PostProcessSettings` (`PostProcessVolume.Settings` _array_element))))
    (bind _output_get (set `local.Mats` _weightedblendables_array))
    (`KismetArrayLibrary.Array_Add` _output_get (make `WeightedBlendable` 1.0 "/Game/Project/Blueprints/Rewind_Effect/TVLineEffect/M_TVLine_Inst.M_TVLine_Inst"))
    (setmembers `PostProcessSettings` :`StructRef` (`PostProcessVolume.Settings` _array_element) :`WeightedBlendables` (make `WeightedBlendables` (`local.Mats`)))))

(fn `UserConstructionScript`)