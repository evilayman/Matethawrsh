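; Trigger box for the Accident3 scenario that marks the machine as safe when an actor enters it while the linked rotating door is open.
; On BeginPlay it caches the first BP_MC actor.
; Any overlap with the door open sets IsMachineSafe on that actor and spawns the safety-on particle effect at a fixed world location.
; An overlap with an invalid cached reference only repeats the lookup.
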(event `self.ReceiveBeginPlay`
  (bind _outactors (`GameplayStatics.GetAllActorsOfClass` "/Game/Project/MainCharacter/BP_MC.BP_MC_C" :!label _label))
  (set `self.MC` (`|GetArrayItem` _outactors)))

(event `self.ReceiveActorBeginOverlap`
  (params (OtherActor :type "Actor Object Reference"))
  (bind _mc (`self.MC`))
  (`/Engine/EditorBlueprintResources/StandardMacros.IsValid` _mc
    (:`Is Valid`
      (if (`/Game/Project/Blueprints/Accident3/MachineAffectedByLever.DoorOpened` (`self.RotatingDoor`))
        (set `/Game/Project/MainCharacter/BP_MC.IsMachineSafe` true _mc)
        (`GameplayStatics.SpawnEmitterAtLocation` "/Game/Project/VFX-Particles/sys_safety_on.sys_safety_on" (409.0 310.0 338.0))))
    (:`Is Not Valid`
      (goto _label))))

(fn `UserConstructionScript`)