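; Level manager actor that coordinates recording and time rewinding for rewindable objects and AI characters.
; On BeginPlay it gathers their rewindable components, registers itself with each Target and creates a record per Target name.
; StartRecord and StopRecord fan out to all components, recording into either a test record or the currently selected one.
; Input releases trigger test recording or a timed rewind, which pauses AI characters before rewinding them.
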(event `self.ReceiveBeginPlay`
  (set `self.TestRecord` (make `/Game/Project/Blueprints/RecordData` (`|MakeArray` (struct) :!type "Transform Structure") (`|MakeArray` (0.0 0.0 0.0) :!type "Vector Structure") (`|MakeArray` (0.0 0.0 0.0) :!type "Vector Structure") (`|MakeArray` (struct) :!type "/Game/Project/Blueprints/SkeletonBoneTransforms Structure") (`|MakeArray` 0.0 :!type "Float (single-precision)")))
  (bind _outactors (`GameplayStatics.GetAllActorsOfClass` "/Game/Project/Blueprints/Deprecated/Targets/Target.Target_C"))
  (for _array_element _outactors
    (set `/Game/Project/Blueprints/Deprecated/Targets/Target.TimeRewinder` self _array_element)
    (`BlueprintMapLibrary.Map_Add` (`self.ActionList`) (`/Game/Project/Blueprints/Deprecated/Targets/Target.Name` _array_element) (make `/Game/Project/Blueprints/RecordData` (`|MakeArray` (struct) :!type "Transform Structure") (`|MakeArray` (0.0 0.0 0.0) :!type "Vector Structure") (`|MakeArray` (0.0 0.0 0.0) :!type "Vector Structure") (`|MakeArray` (struct) :!type "/Game/Project/Blueprints/SkeletonBoneTransforms Structure") (`|MakeArray` 0.0 :!type "Float (single-precision)"))))
  (bind _outactors_2 (`GameplayStatics.GetAllActorsOfClass` "/Game/Project/Blueprints/BP_RewindableObject.BP_RewindableObject_C"))
  (for _array_element_2 _outactors_2
    (`KismetArrayLibrary.Array_Add` (`self.ObjectList`) (`/Game/Project/Blueprints/BP_RewindableObject.RewindableObjectComponent` _array_element_2)))
  (`self.EnableInput` (`GameplayStatics.GetPlayerController` 0))
  (bind _outactors_3 (`GameplayStatics.GetAllActorsOfClass` "/Game/Project/Blueprints/Deprecated/AICharacter.AICharacter_C"))
  (for _array_element_3 _outactors_3
    (`KismetArrayLibrary.Array_Add` (`self.ObjectList`) (`/Game/Project/Blueprints/Deprecated/AICharacter.RewindableAnimatedComponent` _array_element_3))))

(event `InputAction|StartRecording`
  (params (Key :type "Key Structure"))
  (:`Released`
    (`self.StartRecord` true)))

(event `InputAction|StartRewind`
  (params (Key :type "Key Structure"))
  (:`Released`
    (`self.StartRewindEvent`)))

(event `StartRewindEvent`
  (for _array_element (`self.ObjectList`)
    (bind _asaicharacter (cast `/Game/Project/Blueprints/Deprecated/AICharacter` (`ActorComponent.GetOwner` _array_element))
      (:`then`
        (set `/Game/Project/Blueprints/Deprecated/AICharacter.Pause` true _asaicharacter)
        (bind _asrewindable_animated_component (cast `/Game/Project/Blueprints/RewindableAnimatedComponent` _array_element))
        (`/Game/Project/Blueprints/IRewindable.StartRewind` _asrewindable_animated_component (`self.TimeToCompleteRewind`)))
      (:`CastFailed`
        (bind _asrewindable_object_component (cast `/Game/Project/Blueprints/RewindableObjectComponent` _array_element))
        (`/Game/Project/Blueprints/IRewindable.StartRewind` _asrewindable_object_component (`self.TimeToCompleteRewind`))))))

(fn `SetCurrentRecord`
  (params (Name :type String))
  (set `self.CurrentRecord` (`BlueprintMapLibrary.Map_Find` (`self.ActionList`) Name)))

(fn `StartRecord`
  (params (Test :type Boolean :default false))
  (for _array_element (`self.ObjectList`)
    (bind _asrewindable_object_component (cast `/Game/Project/Blueprints/RewindableObjectComponent` _array_element)
      (:`then`
        (if Test
          (`/Game/Project/Blueprints/IRewindable.StartRecording` _asrewindable_object_component (`self.MaxRedundantMoves`) (`self.TestRecord`))
          (else
            (`/Game/Project/Blueprints/IRewindable.StartRecording` _asrewindable_object_component (`self.MaxRedundantMoves`) (`self.CurrentRecord`)))))
      (:`CastFailed`
        (bind _asrewindable_animated_component (cast `/Game/Project/Blueprints/RewindableAnimatedComponent` _array_element))
        (if Test
          (`/Game/Project/Blueprints/IRewindable.StartRecording` _asrewindable_animated_component (`self.MaxRedundantMoves`) (`self.TestRecord`))
          (else
            (`/Game/Project/Blueprints/IRewindable.StartRecording` _asrewindable_animated_component (`self.MaxRedundantMoves`) (`self.CurrentRecord`))))))))

(fn `StopRecord`
  (for _array_element (`self.ObjectList`)
    (bind _asrewindable_object_component (cast `/Game/Project/Blueprints/RewindableObjectComponent` _array_element)
      (:`then`
        (`/Game/Project/Blueprints/RewindableComponent.StopRecording` _asrewindable_object_component))
      (:`CastFailed`
        (bind _asrewindable_animated_component (cast `/Game/Project/Blueprints/RewindableAnimatedComponent` _array_element))
        (`/Game/Project/Blueprints/RewindableComponent.StopRecording` _asrewindable_animated_component)))))

(fn `UserConstructionScript`)