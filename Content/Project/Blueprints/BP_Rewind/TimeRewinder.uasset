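; TimeRewinder is the central manager that records, time-stops and rewinds the level's rewindable objects and characters.
; On BeginPlay it links itself to Shinigami and every BP_Point, then gathers rewindable object and animated components into one list for broadcasting commands.
; Stopping time ends recording and slows global time, offset by Shinigami's custom dilation.
; Resuming restores time and triggers the rewind, including the day-night cycle.
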(event `self.ReceiveBeginPlay`
  (set `/Game/Project/Blueprints/BP_Shinigami.TimeRewinder` self (`self.Shinigami`))
  (set `self.TestRecord` (make `/Game/Project/Blueprints/BP_Rewind/RecordData` (`|MakeArray` (struct) :!type "Transform Structure") (`|MakeArray` (0.0 0.0 0.0) :!type "Vector Structure") (`|MakeArray` (0.0 0.0 0.0) :!type "Vector Structure") (`|MakeArray` (struct) :!type "/Game/Project/Blueprints/BP_Rewind/SkeletonBoneTransforms Structure") (`|MakeArray` 0.0 :!type "Float (single-precision)")))
  (bind _outactors (`GameplayStatics.GetAllActorsOfClass` "/Game/Project/Blueprints/BP_Point.BP_Point_C"))
  (for _array_element _outactors
    (set `/Game/Project/Blueprints/BP_Point.TimeRewinder` self _array_element)
    (set `/Game/Project/Blueprints/BP_Point.Shinigami` (`self.Shinigami`) _array_element)
    (set `/Game/Project/Blueprints/BP_Point.DayAndNightCycle` (`self.DayAndNightCycle`) _array_element))
  (bind _outactors_2 (`GameplayStatics.GetAllActorsOfClass` "/Game/Project/Blueprints/BP_Rewind/BP_RewindableObject.BP_RewindableObject_C"))
  (for _array_element_2 _outactors_2
    (`KismetArrayLibrary.Array_Add` (`self.ObjectList`) (`/Game/Project/Blueprints/BP_Rewind/BP_RewindableObject.RewindableObjectComponent` _array_element_2)))
  (`self.EnableInput` (`GameplayStatics.GetPlayerController` 0))
  (bind _outactors_3 (`GameplayStatics.GetAllActorsOfClass` "/Game/Project/Blueprints/BP_Rewind/BP_RewindableCharacter.BP_RewindableCharacter_C"))
  (for _array_element_3 _outactors_3
    (`KismetArrayLibrary.Array_Add` (`self.ObjectList`) (`/Game/Project/Blueprints/BP_Rewind/BP_RewindableCharacter.RewindableAnimatedComponent` _array_element_3))))

(event `InputAction|StartRecording`
  (params (Key :type "Key Structure"))
  (:`Released`
    (`self.StartRecord` true)))

(event `InputAction|StartRewind`
  (params (Key :type "Key Structure"))
  (:`Released`
    (`self.StartRewindEvent`)))

(event `StartRewindEvent`
  (`/Game/Project/Blueprints/BP_DayAndNightCycle/BP_DayAndNightCycle.OnRewind` (`self.DayAndNightCycle`))
  (for _array_element (`self.ObjectList`)
    (bind _asrewindable_object_component (cast `/Game/Project/Blueprints/BP_Rewind/RewindableObjectComponent` _array_element)
      (:`then`
        (`/Game/Project/Blueprints/BP_Rewind/IRewindable.StartRewind` _asrewindable_object_component (`self.TimeToCompleteRewind`)))
      (:`CastFailed`
        (bind _asrewindable_animated_component (cast `/Game/Project/Blueprints/BP_Rewind/RewindableAnimatedComponent` _array_element))
        (`/Game/Project/Blueprints/BP_Rewind/IRewindable.StartRewind` _asrewindable_animated_component (`self.TimeToCompleteRewind`))))))

(event `StopRecordingEvent`
  (for _array_element (`self.ObjectList`)
    (bind _asrewindable_object_component (cast `/Game/Project/Blueprints/BP_Rewind/RewindableObjectComponent` _array_element)
      (:`then`
        (`/Game/Project/Blueprints/BP_Rewind/RewindableComponent.StopRecording` _asrewindable_object_component))
      (:`CastFailed`
        (bind _asrewindable_animated_component (cast `/Game/Project/Blueprints/BP_Rewind/RewindableAnimatedComponent` _array_element))
        (`/Game/Project/Blueprints/BP_Rewind/RewindableComponent.StopRecording` _asrewindable_animated_component)))))

(event `StopTImeEvent`
  (`self.StopRecordingEvent`)
  (`GameplayStatics.SetGlobalTimeDilation` 0.001)
  (set `Actor.CustomTimeDilation` 1000.0 (`self.Shinigami`)))

(event `ResumeTimeEvent`
  (`GameplayStatics.SetGlobalTimeDilation` 1.0)
  (set `Actor.CustomTimeDilation` 1.0 (`self.Shinigami`))
  (`self.StartRewindEvent`)
  (set `self.WasInRewind` true))

(fn `SetCurrentRecord`
  (params (Name :type String))
  (set `self.CurrentRecord` (`BlueprintMapLibrary.Map_Find` (`self.ActionList`) Name)))

(fn `StartRecord`
  (params (Test :type Boolean :default false))
  (if (`self.WasInRewind`)
    (`/Game/Project/Blueprints/BP_Shinigami.OnRewindComplete` (`self.Shinigami`))
    (set `self.WasInRewind` false))
  (for _array_element (`self.ObjectList`)
    (bind _asrewindable_object_component (cast `/Game/Project/Blueprints/BP_Rewind/RewindableObjectComponent` _array_element)
      (:`then`
        (if Test
          (`/Game/Project/Blueprints/BP_Rewind/IRewindable.StartRecording` _asrewindable_object_component (`self.MaxRedundantMoves`) (`self.TestRecord`))
          (else
            (`/Game/Project/Blueprints/BP_Rewind/IRewindable.StartRecording` _asrewindable_object_component (`self.MaxRedundantMoves`) (`self.CurrentRecord`)))))
      (:`CastFailed`
        (bind _asrewindable_animated_component (cast `/Game/Project/Blueprints/BP_Rewind/RewindableAnimatedComponent` _array_element))
        (if Test
          (`/Game/Project/Blueprints/BP_Rewind/IRewindable.StartRecording` _asrewindable_animated_component (`self.MaxRedundantMoves`) (`self.TestRecord`))
          (else
            (`/Game/Project/Blueprints/BP_Rewind/IRewindable.StartRecording` _asrewindable_animated_component (`self.MaxRedundantMoves`) (`self.CurrentRecord`))))))))

(fn `StopRecord`
  (for _array_element (`self.ObjectList`)
    (bind _asrewindable_object_component (cast `/Game/Project/Blueprints/BP_Rewind/RewindableObjectComponent` _array_element)
      (:`then`
        (`/Game/Project/Blueprints/BP_Rewind/RewindableComponent.StopRecording` _asrewindable_object_component))
      (:`CastFailed`
        (bind _asrewindable_animated_component (cast `/Game/Project/Blueprints/BP_Rewind/RewindableAnimatedComponent` _array_element))
        (`/Game/Project/Blueprints/BP_Rewind/RewindableComponent.StopRecording` _asrewindable_animated_component)))))

(fn `UserConstructionScript`)