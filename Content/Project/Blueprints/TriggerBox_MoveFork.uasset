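; Trigger box that starts a forklift fork move when BP_MC enters, staging either an accident or a safe outcome.
; It checks the IsWearVest flag on a BP_MC reference cached at BeginPlay and passes the matching with- or without-accident position to the ForkLift's MoveForkWithParam.
; An invalid reference on overlap only triggers a new actor lookup, without moving the fork.
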(event `self.ReceiveBeginPlay`
  (bind _outactors (`GameplayStatics.GetAllActorsOfClass` "/Game/Project/MainCharacter/BP_MC.BP_MC_C" :!label _label))
  (set `self.MC` (`|GetArrayItem` _outactors)))

(event `self.ReceiveActorBeginOverlap`
  (params (OtherActor :type "Actor Object Reference"))
  (bind _forklift (`self.ForkLift`))
  (bind _mc (`self.MC`))
  (cast `/Game/Project/MainCharacter/BP_MC` OtherActor)
  (`/Engine/EditorBlueprintResources/StandardMacros.IsValid` _mc
    (:`Is Valid`
      (if (`/Game/Project/MainCharacter/BP_MC.IsWearVest` _mc)
        (`/Game/Project/Blueprints/BP_Forklift.MoveForkWithParam` _forklift (`self.PosWithoutAccident`))
        (else
          (`/Game/Project/Blueprints/BP_Forklift.MoveForkWithParam` _forklift (`self.PosWithAccident`)))))
    (:`Is Not Valid`
      (goto _label))))

(fn `UserConstructionScript`)