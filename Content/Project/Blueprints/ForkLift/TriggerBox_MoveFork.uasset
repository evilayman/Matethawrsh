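; Trigger box that moves a forklift's fork when the BP_MC character walks in, with the outcome depending on whether a vest is worn.
; On overlap it ignores a rewinding character, then sends the fork to the no-accident position with the vest, or the accident position without.
; It caches the first BP_MC at BeginPlay; an invalid reference is only re-fetched, leaving the fork unmoved for that overlap.
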(event `self.ReceiveBeginPlay`
  (bind _outactors (`GameplayStatics.GetAllActorsOfClass` "/Game/Project/MainCharacter/BP_MC.BP_MC_C" :!label _label))
  (set `self.MC` (`|GetArrayItem` _outactors)))

(event `self.ReceiveActorBeginOverlap`
  (params (OtherActor :type "Actor Object Reference"))
  (bind _mc (`self.MC`))
  (bind _forklift (`self.ForkLift`))
  (bind _asbp_mc (cast `/Game/Project/MainCharacter/BP_MC` OtherActor))
  (if (not (`/Game/Project/Blueprints/BP_Rewind/RewindableAnimatedComponent.IsRewinding` (`/Game/Project/Blueprints/BP_Rewind/BP_RewindableCharacter.RewindableAnimatedComponent` _asbp_mc)))
    (`/Engine/EditorBlueprintResources/StandardMacros.IsValid` _mc
      (:`Is Valid`
        (if (`/Game/Project/MainCharacter/BP_MC.IsWearVest` _mc)
          (`/Game/Project/Blueprints/ForkLift/BP_Fork.MoveForkWithParameter` _forklift (`self.PosWithoutAccident`))
          (else
            (`/Game/Project/Blueprints/ForkLift/BP_Fork.MoveForkWithParameter` _forklift (`self.PosWithAccident`)))))
      (:`Is Not Valid`
        (goto _label)))))

(fn `UserConstructionScript`)