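; ConveyorBP is a conveyor that pushes rewindable objects along its forward direction.
; Each tick it takes the actors overlapping its Box and offsets any BP_RewindableObject by the forward vector scaled by Speed and delta time, without sweeping.
; The construction script counter-scales the Arrow component by the actor scale so it keeps a constant size when the conveyor is resized.
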(event `self.ReceiveTick`
  (params (DeltaSeconds :type "Float (single-precision)"))
  (for _array_element (`PrimitiveComponent.GetOverlappingActors` (`self.Box`) null)
    (bind _asbp_rewindable_object (cast `/Game/Project/Blueprints/BP_Rewind/BP_RewindableObject` _array_element))
    (`self.K2_AddActorWorldOffset` _asbp_rewindable_object (* (`KismetMathLibrary.GetForwardVector` (`self.K2_GetActorRotation`)) (* DeltaSeconds (`self.Speed`))) false false)))

(fn `UserConstructionScript`
  (`SceneComponent.SetRelativeScale3D` (`self.Arrow`) (/ (1.0 1.0 1.0) (`self.GetActorScale3D`))))