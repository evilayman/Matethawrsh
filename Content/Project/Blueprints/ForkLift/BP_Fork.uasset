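; Forklift actor that drives to a requested position and works with the game's rewind mechanic.
; MoveForkWithParameter plays an attached engine sound, then a timeline lerps the actor from its current location to the target without sweep while spinning the four wheels.
; While RewindableObjectComponent reports RewindStarted, Tick spins the wheels backward by a fixed per-frame step, not scaled by delta time.
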(event `MoveForkWithParameter`
  (params (NewPosition :type "Vector Structure"))
  (`GameplayStatics.SpawnSoundAttached` "/Game/Project/SFX/A6_forklift.A6_forklift" (`self.RightWheel_Front`) "None" (0.0 0.0 0.0) (struct) "KeepRelativeOffset" false 0.3 1.0 0.0 "/Game/Project/Sounds/VoiceAttenuation.VoiceAttenuation" null)
  (bind _output_get (set `self.ForkStartPosParam` (`self.K2_GetActorLocation`)))
  (bind (_direction _alpha) (`Timeline|MoveFork` :!via `PlayFromStart`)
    (:`Update`
      (`self.K2_SetActorLocation` (`KismetMathLibrary.VLerp` _output_get NewPosition _alpha))
      (`SceneComponent.K2_AddLocalRotation` (`self.RightWheel_Front`) (struct :`Roll` 5.0) false false)
      (`SceneComponent.K2_AddLocalRotation` (`self.LeftWheel_Back`) (struct :`Roll` 5.0) false false)
      (`SceneComponent.K2_AddLocalRotation` (`self.RightWheel_Back`) (struct :`Roll` 5.0) false false)
      (`SceneComponent.K2_AddLocalRotation` (`self.LeftWheel_Front`) (struct :`Roll` 5.0) false false))))

(event `self.ReceiveTick`
  (params (DeltaSeconds :type "Float (single-precision)"))
  (`parent.ReceiveTick` DeltaSeconds)
  (if (`/Game/Project/Blueprints/BP_Rewind/RewindableObjectComponent.RewindStarted` (`self.RewindableObjectComponent`))
    (`SceneComponent.K2_AddLocalRotation` (`self.RightWheel_Front`) (struct :`Roll` -5.0) false false)
    (`SceneComponent.K2_AddLocalRotation` (`self.LeftWheel_Back`) (struct :`Roll` -5.0) false false)
    (`SceneComponent.K2_AddLocalRotation` (`self.RightWheel_Back`) (struct :`Roll` -5.0) false false)
    (`SceneComponent.K2_AddLocalRotation` (`self.LeftWheel_Front`) (struct :`Roll` -5.0) false false)))

(fn `UserConstructionScript`)