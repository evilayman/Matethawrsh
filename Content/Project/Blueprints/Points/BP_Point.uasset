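; Waypoint actor that scripts what a rewindable character does on reaching it, in forward play or during rewind.
; Both arrival events store the character, and for BP_MC also cache it and clear its work-done flag.
; Helper functions relay movement, turn, look, speech, bone simulation and state commands to characters, using actor-relative location offsets.
; Others drive time recording and rewind, redirect to RewindPoint, summon the Shinigami or trigger side-character panic.
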(event `OnPointArrive`
  (params (RewindableCharacter :type "/Game/Project/Blueprints/BP_Rewind/BP_RewindableCharacter Object Reference"))
  (set `self.RewindableCharacter` RewindableCharacter)
  (bind _asbp_mc (cast `/Game/Project/MainCharacter/BP_MC` (`self.RewindableCharacter`)))
  (set `self.MC` _asbp_mc)
  (`self.SetWorkDone` false))

(event `OnPointArriveRewind`
  (params (`Rewindable Character` :type "/Game/Project/Blueprints/BP_Rewind/BP_RewindableCharacter Object Reference"))
  (set `self.RewindableCharacter` `Rewindable Character`)
  (bind _asbp_mc (cast `/Game/Project/MainCharacter/BP_MC` (`self.RewindableCharacter`)))
  (set `self.MC` _asbp_mc)
  (`self.SetWorkDone` false))

(fn `LookAtActor`
  (params (LookActor :type "Actor Object Reference") (LookDuration :type "Float (double-precision)" :default 1.0))
  (`/Game/Project/Blueprints/BP_Rewind/BP_RewindableCharacter.LookAtActor` (`self.RewindableCharacter`) LookActor LookDuration))

(fn `LookAtLocation`
  (params (LookDuration :type "Float (double-precision)" :default 1.0))
  (`/Game/Project/Blueprints/BP_Rewind/BP_RewindableCharacter.LookAtLocation` (`self.RewindableCharacter`) (+ (`self.LookLocation`) (`self.K2_GetActorLocation`)) LookDuration))

(fn `LookAtPlayer`
  (params (LookDuration :type "Float (double-precision)" :default 1.0))
  (`/Game/Project/Blueprints/BP_Rewind/BP_RewindableCharacter.LookAtActor` (`self.RewindableCharacter`) (`GameplayStatics.GetPlayerController` 0) LookDuration))

(fn `MoveOn`
  (params (Speed :type "Float (double-precision)" :default 150.0))
  (`/Game/Project/Blueprints/BP_Rewind/BP_RewindableCharacter.MoveToPoint` (`self.RewindableCharacter`) (`self.NextPoint`) Speed)
  (`/Engine/EditorBlueprintResources/StandardMacros.IsValid` (`self.MC`)
    (:`Is Valid`
      (`/Game/Project/Blueprints/BP_Rewind/TimeRewinder.StartRecord` (`self.TimeRewinder`) false))))

(fn `MoveToPanic`
  (`/Game/Project/Blueprints/BP_SideCharacterManager.MoveToPanic` (`self.SideCharacterManager`)))

(fn `MoveToPoint`
  (params (Speed :type "Float (double-precision)" :default 100.0))
  (`/Game/Project/Blueprints/BP_Rewind/BP_RewindableCharacter.MoveToPoint` (`self.RewindableCharacter`) (`self.NextPoint`) Speed))

(fn `Rewind`
  (set `/Game/Project/Blueprints/BP_Rewind/BP_RewindableCharacter.NextPoint` (`self.RewindPoint`) (`self.RewindableCharacter`))
  (`/Game/Project/Blueprints/BP_Rewind/TimeRewinder.StartRewindEvent` (`self.TimeRewinder`)))

(fn `SetActiveState`
  (params (ActiveState :type Integer))
  (`/Game/Project/Blueprints/BP_Rewind/BP_RewindableCharacter.SetActiveState` (`self.RewindableCharacter`) ActiveState))

(fn `SetWorkDone`
  (params (IsWorkDone :type Boolean))
  (set `/Game/Project/Blueprints/BP_Rewind/BP_RewindableCharacter.isWorkingDone` IsWorkDone (`self.RewindableCharacter`)))

(fn `SimulateBones`
  (params (BlendWeight :type "Float (double-precision)" :default 1.0))
  (`/Game/Project/Blueprints/BP_Rewind/BP_RewindableCharacter.SimulateBones` (`self.RewindableCharacter`) BlendWeight))

(fn `Speak`
  (params (TargetCharacter :type "/Game/Project/Blueprints/Characters Enum" :default "NewEnumerator3") (Sound :type "SoundBase Object Reference"))
  (bind _sidecharactermanager (`self.SideCharacterManager`))
  (switch `/Game/Project/Blueprints/Characters` TargetCharacter
    (:`NewEnumerator3`
      (`/Game/Project/Blueprints/BP_Rewind/BP_RewindableCharacter.Speak` (`self.RewindableCharacter`) Sound))
    (:`NewEnumerator0`
      (`/Game/Project/Blueprints/BP_Rewind/BP_RewindableCharacter.Speak` (`/Game/Project/Blueprints/BP_SideCharacterManager.MC` _sidecharactermanager) Sound))
    (:`NewEnumerator1`
      (`/Game/Project/Blueprints/BP_Rewind/BP_RewindableCharacter.Speak` (`/Game/Project/Blueprints/BP_SideCharacterManager.SC_1` _sidecharactermanager) Sound))
    (:`NewEnumerator2`
      (`/Game/Project/Blueprints/BP_Rewind/BP_RewindableCharacter.Speak` (`/Game/Project/Blueprints/BP_SideCharacterManager.SC_2` _sidecharactermanager) Sound))))

(fn `SummonShinigami`
  (params (Accident :type "/Game/Project/Blueprints/Enum_Shinigami Enum" :default "NewEnumerator6"))
  (`/Game/Project/Blueprints/BP_Shinigami.OnSummon` (`self.Shinigami`) Accident (+ (`self.ShinigamiLocation`) (`self.K2_GetActorLocation`)))
  (set `/Game/Project/Blueprints/BP_Rewind/BP_RewindableCharacter.NextPoint` (`self.RewindPoint`) (`self.RewindableCharacter`)))

(fn `TurnToActor`
  (params (TurnActor :type "Actor Object Reference") (BreakFocusTime :type "Float (double-precision)" :default 1.0))
  (`/Game/Project/Blueprints/BP_Rewind/BP_RewindableCharacter.TurnToActor` (`self.RewindableCharacter`) TurnActor true BreakFocusTime))

(fn `TurnToLocation`
  (params (BreakFocusTime :type "Float (double-precision)" :default 1.0))
  (`/Game/Project/Blueprints/BP_Rewind/BP_RewindableCharacter.TurnToLocation` (`self.RewindableCharacter`) (+ (`self.TurnLocation`) (`self.K2_GetActorLocation`)) true BreakFocusTime))

(fn `TurnToPlayer`
  (params (BreakFocusTime :type "Float (double-precision)" :default 1.0))
  (`/Game/Project/Blueprints/BP_Rewind/BP_RewindableCharacter.TurnToActor` (`self.RewindableCharacter`) (`GameplayStatics.GetPlayerController` 0) true BreakFocusTime))

(fn `UserConstructionScript`)