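; BP_Paper is a pickup paper item in the safety equipment set that reports its use to the tutorial.
; Pickup runs the parent logic, then sets a fixed relative offset and flip on the mesh, while Drop arms a Droped flag.
; An actor overlap, or the first mesh hit after a drop, clears the flag and calls TutorialPoint.PaperUsed, passing true only when the other actor is a TriggerBox.
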(event `self.ReceiveBeginPlay`
  (`parent.ReceiveBeginPlay`)
  (set `self.Droped` false))

(event `self.ReceiveActorBeginOverlap`
  (params (OtherActor :type "Actor Object Reference"))
  (bind _tutorialpoint (`self.TutorialPoint`))
  (`parent.ReceiveActorBeginOverlap` OtherActor)
  (set `self.Droped` false)
  (cast `TriggerBox` OtherActor
    (:`then`
      (`/Game/Project/Blueprints/Points/MC_Tutorial.PaperUsed` _tutorialpoint true))
    (:`CastFailed`
      (`/Game/Project/Blueprints/Points/MC_Tutorial.PaperUsed` _tutorialpoint false))))

(event `/Game/VirtualRealityBP/Blueprints/PickupActorInterface.Pickup`
  (params (AttachTo :type "SceneComponent Object Reference"))
  (`parent.Pickup` AttachTo)
  (`SceneComponent.K2_SetRelativeLocationAndRotation` (`self.StaticMeshComponent`) (0.000388 -43.142677 -6.992931) (struct :`Yaw` 180.0) false false))

(event `/Game/VirtualRealityBP/Blueprints/PickupActorInterface.Drop`
  (`parent.Drop`)
  (set `self.Droped` true))

(event `self.StaticMeshComponent.OnComponentHit`
  (params (HitComponent :type "PrimitiveComponent Object Reference") (OtherActor :type "Actor Object Reference") (OtherComp :type "PrimitiveComponent Object Reference") (NormalImpulse :type "Vector Structure") (Hit :type "HitResult Structure (by ref)"))
  (bind _tutorialpoint (`self.TutorialPoint`))
  (if (`self.Droped`)
    (set `self.Droped` false)
    (cast `TriggerBox` OtherActor
      (:`then`
        (`/Game/Project/Blueprints/Points/MC_Tutorial.PaperUsed` _tutorialpoint true))
      (:`CastFailed`
        (`/Game/Project/Blueprints/Points/MC_Tutorial.PaperUsed` _tutorialpoint false)))))

(fn `UserConstructionScript`
  (`parent.UserConstructionScript`))