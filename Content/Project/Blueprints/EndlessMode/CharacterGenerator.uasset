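; Endless mode spawner that sends characters to randomly chosen free glove, eyewear and hat points, then an exit.
; It spawns rotating character classes at random positions up to a cap, retrying after a delay, and pauses during rewind.
; Each character registers with the TimeRewinder and receives reserved points with random work times.
; Score updates the score widget and selects difficulty tiers controlling cap, spawn rate, item-count odds and work times.
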(event `self.ReceiveBeginPlay`
  (`self.ResetScore`)
  (`self.TryGenerate`))

(event `TryGenerate`
  (bind _spawnedcharacter (`self.SpawnedCharacter`))
  ;[1 1 1] Check if you can spawn
  (if (and (< (`self.CharactersCount`) (`self.MaxCharacters`)) (`self.CanSpawn`) (not (`/Game/Project/Blueprints/BP_Rewind/TimeRewinder.IsRewinding` (`self.TimeRewinder`))))
    (`self.GetNumberOfItems`)
    (bind _succeeded (`self.GetPointList`))
    (if _succeeded
      (`self.SpawnCharacter`)
      (for _array_element (`self.SelectedPoints`)
        (`KismetArrayLibrary.Array_Add` (`/Game/Project/Blueprints/EndlessMode/BP_EndlessCharacter.Points` _spawnedcharacter) _array_element))
      (for _array_element_2 (`self.SelectedPointsTimes`)
        (`KismetArrayLibrary.Array_Add` (`/Game/Project/Blueprints/EndlessMode/BP_EndlessCharacter.PointsTimes` _spawnedcharacter) _array_element_2))
      (`/Game/Project/Blueprints/EndlessMode/BP_EndlessCharacter.PointDone` (`self.SpawnedCharacter`)))))

(event `SpawnCharacter`
  ;[1 1 1] Spawn Character
  (bind _characterclass (`self.GetCharacterClass`))
  (bind _spawntransform (`self.GetSpawnPosition`))
  (bind _returnvalue (`|SpawnActorFromClass` _characterclass _spawntransform "AdjustIfPossibleButAlwaysSpawn" "OverrideRootScale" null null))
  (bind _output_get (set `self.SpawnedCharacter` _returnvalue))
  (`/Game/Project/Blueprints/BP_Rewind/TimeRewinder.AddRewindableAnimatedObject` (`self.TimeRewinder`) (`/Game/Project/Blueprints/BP_Rewind/BP_RewindableCharacter.RewindableAnimatedComponent` _output_get))
  (set `/Game/Project/Blueprints/EndlessMode/BP_EndlessCharacter.CharacterGenerator` self _output_get)
  (`/Engine/EditorBlueprintResources/StandardMacros.IncrementInt` (`self.CharactersCount`)
    (:`  `
      (set `self.CanSpawn` false)
      (`KismetSystemLibrary.Delay` (`self.SpawnRate`))
      (set `self.CanSpawn` true)
      (`self.TryGenerate`))))

(fn `GetAvailablePoint`
  (params (Points :type "Array of /Game/Project/Blueprints/Points/BP_Point Object Reference"))
  (returns (AvailablePoint :type "/Game/Project/Blueprints/Points/BP_Point Object Reference"))
  (bind _temppoints (`self.TempPoints`))
  (bind _returnvalue (`KismetArrayLibrary.Array_Length` _temppoints))
  (`KismetArrayLibrary.Array_Clear` (`self.TempPoints`))
  (for _array_element Points
    (if (not (`/Game/Project/Blueprints/Points/BP_Point.IsActive` _array_element))
      (`KismetArrayLibrary.Array_Add` (`self.TempPoints`) _array_element)))
  (if (> _returnvalue 0)
    (return (`|GetArrayItem` _temppoints (`KismetMathLibrary.RandomIntegerInRange` 0 (- _returnvalue 1))))
    (else
      (return null))))

(fn `GetAvailablePoints`
  (`KismetArrayLibrary.Array_Clear` (`self.AvailablePoints`))
  (bind _availablepoint (`self.GetAvailablePoint` (`self.GlovePoints`)))
  (`/Engine/EditorBlueprintResources/StandardMacros.IsValid` _availablepoint
    (:`Is Valid`
      (`KismetArrayLibrary.Array_Add` (`self.AvailablePoints`) _availablepoint))
    (:`Is Not Valid`
      _))
  (bind _availablepoint_2 (`self.GetAvailablePoint` (`self.EyewarePoints`)))
  (`/Engine/EditorBlueprintResources/StandardMacros.IsValid` _availablepoint_2
    (:`Is Valid`
      (`KismetArrayLibrary.Array_Add` (`self.AvailablePoints`) _availablepoint_2))
    (:`Is Not Valid`
      _))
  (bind _availablepoint_3 (`self.GetAvailablePoint` (`self.HatPoints`)))
  (`/Engine/EditorBlueprintResources/StandardMacros.IsValid` _availablepoint_3
    (:`Is Valid`
      (`KismetArrayLibrary.Array_Add` (`self.AvailablePoints`) _availablepoint_3))))

(fn `GetCharacterClass`
  (returns (CharacterClass :type "/Game/Project/Blueprints/EndlessMode/BP_EndlessCharacter Class Reference"))
  (bind _currentcharacter (`self.CurrentCharacter`))
  (`/Engine/EditorBlueprintResources/StandardMacros.IncrementInt` _currentcharacter
    (:`  `
      (if (not (< _currentcharacter (`KismetArrayLibrary.Array_Length` (`self.EndlessCharacters`))))
        (set `self.CurrentCharacter` 0))
      (return (`|GetArrayItem` (`self.EndlessCharacters`) (`self.CurrentCharacter`))))))

(fn `GetNumberOfItems`
  (bind _returnvalue (`KismetMathLibrary.RandomFloatInRange` 1.0 100.0))
  (bind _oneitempercentage (`self.OneItemPercentage`))
  (bind _returnvalue_2 (+ (`self.OneItemPercentage`) (`self.TwoItemPercentage`)))
  (if (and (> _returnvalue 0.0) (<= _returnvalue (`self.OneItemPercentage`)))
    (set `self.ItemCount` 1)
    (elif (and (> _returnvalue _oneitempercentage) (<= _returnvalue (+ _oneitempercentage (`self.TwoItemPercentage`))))
      (set `self.ItemCount` 2)
      (elif (and (> _returnvalue _returnvalue_2) (<= _returnvalue (+ _returnvalue_2 (`self.ThreeItemPercentage`))))
        (set `self.ItemCount` 3)
        (else
          (set `self.ItemCount` 1))))))

(fn `GetPointList`
  (returns (Succeeded :type Boolean))
  (locals (pointCondition :type Boolean))
  (`self.GetAvailablePoints`)
  (bind _output_get (set `local.pointCondition` (>= (`KismetArrayLibrary.Array_Length` (`self.AvailablePoints`)) (`self.ItemCount`))))
  (if _output_get
    (`self.SelectPoints`))
  (return (`local.pointCondition`)))

(fn `GetSpawnPosition`
  (returns (SpawnTransform :type "Transform Structure"))
  (return (`KismetMathLibrary.MakeTransform` (+ (`|GetArrayItem` (`self.SpawnPositions`) (`KismetMathLibrary.RandomIntegerInRange` 0 (- (`KismetArrayLibrary.Array_Length` (`self.SpawnPositions`)) 1))) (`self.K2_GetActorLocation`)))))

(fn `IncreaseScore`
  (bind _result (`/Engine/EditorBlueprintResources/StandardMacros.IncrementInt` (`self.Score`))
    (:`  `
      (`self.UpdateDifficultySetting`)
      (bind _asw_score (cast `/Game/Project/Widgets/W_Score` (`WidgetComponent.GetUserWidgetObject` (`self.Widget`))))
      (`/Game/Project/Widgets/W_Score.UpdateScore` _asw_score _result))))

(fn `ResetScore`
  (bind _output_get (set `self.Score` 0))
  (`self.UpdateDifficultySetting`)
  (bind _asw_score (cast `/Game/Project/Widgets/W_Score` (`WidgetComponent.GetUserWidgetObject` (`self.Widget`))))
  (`/Game/Project/Widgets/W_Score.UpdateScore` _asw_score _output_get))

(fn `SelectPoints`
  (bind _availablepoints (`self.AvailablePoints`))
  (`KismetArrayLibrary.Array_Clear` (`self.SelectedPointsTimes`))
  (`KismetArrayLibrary.Array_Clear` (`self.SelectedPoints`))
  (for _ (range 1 (+ (`self.ItemCount`) 1))
    (bind _output_get (set `self.RandomSelectedPoint` (`KismetMathLibrary.RandomIntegerInRange` 0 (- (`KismetArrayLibrary.Array_Length` _availablepoints) 1))))
    (bind _output (`|GetArrayItem` _availablepoints _output_get))
    (`KismetArrayLibrary.Array_Add` (`self.SelectedPoints`) _output)
    (set `/Game/Project/Blueprints/Points/BP_Point.IsActive` true _output)
    (`KismetArrayLibrary.Array_RemoveItem` (`self.AvailablePoints`) _output)
    (`KismetArrayLibrary.Array_Add` (`self.SelectedPointsTimes`) (`KismetMathLibrary.RandomFloatInRange` (`self.WorkTimeMin`) (`self.WorkTimeMax`))))
  (`KismetArrayLibrary.Array_Add` (`self.SelectedPoints`) (`|GetArrayItem` (`self.ExitPoints`) (`KismetMathLibrary.RandomIntegerInRange` 0 (- (`KismetArrayLibrary.Array_Length` (`self.ExitPoints`)) 1)))))

(fn `SetDifficultySetting`
  (params (Difficulty :type "/Game/Project/Blueprints/EndlessMode/GeneratorSettings Structure"))
  (bind (_score _maxcharacters _spawnrate _oneitempercentage _twoitempercentage _threeitempercentage _worktimemin _worktimemax) (break `/Game/Project/Blueprints/EndlessMode/GeneratorSettings` Difficulty))
  (set `self.MaxCharacters` _maxcharacters)
  (set `self.SpawnRate` _spawnrate)
  (set `self.OneItemPercentage` _oneitempercentage)
  (set `self.TwoItemPercentage` _twoitempercentage)
  (set `self.ThreeItemPercentage` _threeitempercentage)
  (set `self.WorkTimeMin` _worktimemin)
  (set `self.WorkTimeMax` _worktimemax))

(fn `UpdateDifficultySetting`
  (locals (IsUpdated :type Boolean))
  (bind _difficultysettings (`self.DifficultySettings`))
  (set `local.IsUpdated` false)
  (for _array_element (`self.DifficultySettings`)
    (if (<= (`self.Score`) (`.Score_2_01962E694F5E5165D2992CB1CBBF1A41` (break `/Game/Project/Blueprints/EndlessMode/GeneratorSettings` _array_element)))
      (set `local.IsUpdated` true)
      (`self.SetDifficultySetting` _array_element)
      (break)))
  (if (`local.IsUpdated`)
    _
    (elif (> (`KismetArrayLibrary.Array_Length` _difficultysettings) 0)
      (`self.SetDifficultySetting` (`|GetArrayItem` _difficultysettings (`KismetArrayLibrary.Array_LastIndex` _difficultysettings))))))

(fn `UserConstructionScript`)