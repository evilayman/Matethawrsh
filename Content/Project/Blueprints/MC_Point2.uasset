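; MC_Point2 is a waypoint Blueprint for a rewindable character, acting as a checkpoint that depends on whether the character is safe.
; On arrival, a safe character moves on to NextPoint while TimeRewinder starts recording.
; An unsafe one dies, then after a short delay its next point becomes RewindPoint and TimeRewinder starts a rewind.
; Arrival during a rewind always resumes movement to NextPoint and recording.
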(event `self.OnPointArrive`
  (params (RewindableCharacter :type "/Game/Project/Blueprints/BP_Rewind/BP_RewindableCharacter Object Reference"))
  (`parent.OnPointArrive` RewindableCharacter)
  (if (`/Game/Project/Blueprints/BP_Rewind/BP_RewindableCharacter.IsSafe` (`self.RewindableCharacter`))
    (`/Game/Project/Blueprints/BP_Rewind/BP_RewindableCharacter.MoveToNextPoint` (`self.RewindableCharacter`) (`self.NextPoint`))
    (`/Game/Project/Blueprints/BP_Rewind/TimeRewinder.StartRecord` (`self.TimeRewinder`) false)
    (else
      (`/Game/Project/Blueprints/BP_Rewind/BP_RewindableCharacter.Die` (`self.RewindableCharacter`) 1.0)
      (`KismetSystemLibrary.Delay` 2.0)
      (set `/Game/Project/Blueprints/BP_Rewind/BP_RewindableCharacter.NextPoint` (`self.RewindPoint`) (`self.RewindableCharacter`))
      (`/Game/Project/Blueprints/BP_Rewind/TimeRewinder.StartRewindEvent` (`self.TimeRewinder`)))))

(event `self.OnPointArriveRewind`
  (params (`Rewindable Character` :type "/Game/Project/Blueprints/BP_Rewind/BP_RewindableCharacter Object Reference"))
  (`parent.OnPointArriveRewind` `Rewindable Character`)
  (`/Game/Project/Blueprints/BP_Rewind/BP_RewindableCharacter.MoveToNextPoint` (`self.RewindableCharacter`) (`self.NextPoint`))
  (`/Game/Project/Blueprints/BP_Rewind/TimeRewinder.StartRecord` (`self.TimeRewinder`) false))

(fn `UserConstructionScript`
  (`parent.UserConstructionScript`))