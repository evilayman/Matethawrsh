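; MC_Accident4 is a path point that stages a welding accident for a rewindable character.
; On arrival it sets the active state, makes the welding gun the character's target object and marks the work done after a delay.
; If MC wears eyewear, it resets the state and moves on; otherwise the character drops the object and a Shinigami is summoned.
; Arriving during rewind simply moves on.
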(event `self.OnPointArrive`
  (params (RewindableCharacter :type "/Game/Project/Blueprints/BP_Rewind/BP_RewindableCharacter Object Reference"))
  (`parent.OnPointArrive` RewindableCharacter)
  (`self.SetActiveState` (`self.ActiveState`))
  (set `/Game/Project/Blueprints/BP_Rewind/BP_RewindableCharacter.TargetObject` (`self.WeldingGun`) (`self.RewindableCharacter`))
  (`KismetSystemLibrary.Delay` 5.0)
  (`self.SetWorkDone` true)
  (if (`/Game/Project/Blueprints/BP_MC.IsWearEyeWear` (`self.MC`))
    (`KismetSystemLibrary.Delay` 7.0)
    (`self.SetActiveState` 0)
    (`KismetSystemLibrary.Delay` 1.0)
    (`self.MoveOn` 150.0)
    (else
      (`KismetSystemLibrary.Delay` 3.0)
      (`/Game/Project/Blueprints/BP_Rewind/BP_RewindableCharacter.DropObject` (`self.RewindableCharacter`))
      (`self.SummonShinigami` "NewEnumerator6"))))

(event `self.OnPointArriveRewind`
  (params (`Rewindable Character` :type "/Game/Project/Blueprints/BP_Rewind/BP_RewindableCharacter Object Reference"))
  (`parent.OnPointArriveRewind` `Rewindable Character`)
  (`self.MoveOn` 100.0))

(fn `UserConstructionScript`
  (`parent.UserConstructionScript`))