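; TestPoint is a point Blueprint that reacts when a rewindable character arrives, apparently as a test.
; It extends its parent's forward and rewind arrival events, calling MoveOn with a fixed value in both.
; Forward arrival also makes the referenced Gloves pickable and sets their static mesh to Movable, while rewind arrival leaves the Gloves untouched.
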(event `self.OnPointArrive`
  (params (RewindableCharacter :type "/Game/Project/Blueprints/BP_Rewind/BP_RewindableCharacter Object Reference"))
  (bind _gloves (`self.Gloves`))
  (`parent.OnPointArrive` RewindableCharacter)
  (`self.MoveOn` 150.0)
  (set `/Game/Project/Blueprints/SafetyEquipments/BP_GLOVES_gloves_2.CanBePickedUp` true _gloves)
  (`SceneComponent.SetMobility` (`StaticMeshActor.StaticMeshComponent` _gloves) "Movable"))

(event `self.OnPointArriveRewind`
  (params (`Rewindable Character` :type "/Game/Project/Blueprints/BP_Rewind/BP_RewindableCharacter Object Reference"))
  (`parent.OnPointArriveRewind` `Rewindable Character`)
  (`self.MoveOn` 150.0))

(fn `UserConstructionScript`
  (`parent.UserConstructionScript`))