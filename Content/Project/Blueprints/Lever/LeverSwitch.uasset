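; LeverSwitch is a physics-driven two-position lever that rotates a linked machine up or down.
; Each tick it reads the Handle's pitch in actor space, treating negative pitch as on.
; Unless ReturnToNormalOnRelease is set, it retargets the PhysicsConstraint's angular drive toward the side the handle leans, making it bistable.
; When the state flips, it calls RotateTheMachine on the LinkedObject, cast to MachineAffectedByLever.
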(event `self.ReceiveTick`
  (params (DeltaSeconds :type "Float (single-precision)"))
  (bind _returnvalue (< (.pitch (`KismetMathLibrary.InverseTransformRotation` (`self.GetTransform`) (`SceneComponent.K2_GetComponentRotation` (`self.Handle`)))) 0.0))
  (if (not (`self.ReturnToNormalOnRelease`))
    (`PhysicsConstraintComponent.SetAngularOrientationTarget` (`self.PhysicsConstraint`) (`KismetMathLibrary.MakeRotator` 0.0 (select `bool` _returnvalue :`false` 45.0 :`true` -45.0 :!type "Float (single-precision)"))))
  (if (!= (`self.On`) _returnvalue)
    (bind _output_get (set `self.On` _returnvalue))
    (if _output_get
      (bind _asmachine_affected_by_lever (cast `/Game/Project/Blueprints/Lever/MachineAffectedByLever` (`self.LinkedObject`)))
      (`/Game/Project/Blueprints/Lever/MachineAffectedByLever.RotateTheMachine` _asmachine_affected_by_lever "Up")
      (else
        (bind _asmachine_affected_by_lever_2 (cast `/Game/Project/Blueprints/Lever/MachineAffectedByLever` (`self.LinkedObject`)))
        (`/Game/Project/Blueprints/Lever/MachineAffectedByLever.RotateTheMachine` _asmachine_affected_by_lever_2 "Down")))))

(fn `UserConstructionScript`)