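; Interactive push button that opens a left and a right door when a component overlaps it.
; The first overlapping component is tracked and its start location stored, and both doors receive an open message immediately, with no close message sent.
; Each tick, that component's travel along the button base's local Z sets the clamped press depth.
; Once the tracked overlap ends, the button interpolates back toward rest.
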(event `Key|E`
  (params (Key :type "Key Structure")))

(event `self.Button_Component.OnComponentBeginOverlap`
  (params (OverlappedComponent :type "PrimitiveComponent Object Reference") (OtherActor :type "Actor Object Reference") (OtherComp :type "PrimitiveComponent Object Reference") (OtherBodyIndex :type Integer) (bFromSweep :type Boolean) (SweepResult :type "HitResult Structure (by ref)"))
  (`/Engine/EditorBlueprintResources/StandardMacros.IsValid` (`self.OverlappedComponent`)
    (:`Is Not Valid`
      (bind _output_get (set `self.OverlappedComponent` OtherComp))
      (set `self.InitialOverlapLocation` (`SceneComponent.K2_GetComponentLocation` _output_get))
      (message `/Game/Project/Blueprints/FactoryDoors/iDoorOpened.OpenDoor` (`self.LeftDoor`))
      (message `/Game/Project/Blueprints/FactoryDoors/iDoorOpened.OpenDoor` (`self.RightDoor`)))))

(event `self.Button_Component.OnComponentEndOverlap`
  (params (OverlappedComponent :type "PrimitiveComponent Object Reference") (OtherActor :type "Actor Object Reference") (OtherComp :type "PrimitiveComponent Object Reference") (OtherBodyIndex :type Integer))
  (if (== OtherComp (`self.OverlappedComponent`))
    (set `self.OverlappedComponent` null)))

(event `self.ReceiveTick`
  (params (DeltaSeconds :type "Float (single-precision)"))
  (bind _button_component (`self.Button_Component`))
  (bind _button_base (`self.Button_Base`))
  (bind (_returnvalue_x _returnvalue_y _returnvalue_z) (`KismetMathLibrary.BreakVector` (- (`KismetMathLibrary.InverseTransformLocation` (`SceneComponent.K2_GetComponentToWorld` _button_base) (`self.InitialOverlapLocation`)) (`KismetMathLibrary.InverseTransformLocation` (`SceneComponent.K2_GetComponentToWorld` _button_base) (`SceneComponent.K2_GetComponentLocation` (`self.OverlappedComponent`))))))
  (`|ExecutionSequence`
    (:`then_0`
      (`/Engine/EditorBlueprintResources/StandardMacros.IsValid` (`self.OverlappedComponent`)
        (:`Is Valid`
          (bind _output_get (set `self.ButtonPressAmount` (`KismetMathLibrary.FClamp` _returnvalue_z 0.0 (`self.MaxButtonPressedAmount`))))
          (`SceneComponent.K2_SetRelativeLocation` _button_component (`KismetMathLibrary.MakeVector` 0.0 0.0 (* _output_get -1.0)) false false))
        (:`Is Not Valid`
          (`SceneComponent.K2_SetRelativeLocation` _button_component (`KismetMathLibrary.VInterpTo` (`SceneComponent.RelativeLocation` _button_component) (0.0 0.0 0.0) DeltaSeconds) false false))))))

(fn `UserConstructionScript`)