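; Day and night cycle Blueprint that rotates a light and keeps the sky sphere's sun direction in sync.
; Tick pitches the light at a set speed while the cycle is moving, and NewPointReached saves its current rotation.
; OnRewind pauses the cycle and plays a timeline that sets the pitch to the saved value scaled by a curve, then resumes the cycle when finished.
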(event `self.ReceiveBeginPlay`
  (set `self.CycleMove` true))

(event `NewPointReached`
  (set `self.LastPointLightRotation` (`self.K2_GetActorRotation` (`self.Light`))))

(event `OnRewind`
  (set `self.CycleMove` false)
  (bind (_direction _angle) (`Timeline|RewindReverseDayNightCycle` :`NewTime` (`self.RewindTime`))
    (:`Update`
      (`self.K2_SetActorRotation` (`self.Light`) (`KismetMathLibrary.MakeRotator` 0.0 (* (.z _angle) (.pitch (`self.LastPointLightRotation`)))) false)
      (`/Engine/EngineSky/BP_Sky_Sphere.UpdateSunDirection` (`self.SkySphere`)))
    (:`Finished`
      (set `self.CycleMove` true))))

(event `self.ReceiveTick`
  (params (DeltaSeconds :type "Float (single-precision)"))
  (if (`self.CycleMove`)
    (`self.K2_AddActorLocalRotation` (`self.Light`) (`KismetMathLibrary.MakeRotator` 0.0 (* DeltaSeconds (`self.Speed`))) false false)
    (`/Engine/EngineSky/BP_Sky_Sphere.UpdateSunDirection` (`self.SkySphere`))))

(fn `UserConstructionScript`)