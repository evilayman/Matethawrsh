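; HandleMotionControllerRayDrawing toggles the laser pointer meshes on both VR motion controllers according to game state.
; Shortly after BeginPlay it gets the player's MotionControllerPawn and hides both lasers.
; Tick repeatedly binds to Accident6's YouWon and Shinigami's GameOver events, rather than binding once.
; Either event leads to the same logic, which makes both lasers visible again.
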(event `self.ReceiveBeginPlay`
  (`KismetSystemLibrary.Delay` 0.2)
  (bind _asmotion_controller_pawn (cast `/Game/VirtualRealityBP/Blueprints/MotionControllerPawn` (`GameplayStatics.GetPlayerPawn` 0)))
  (`SceneComponent.SetVisibility` (`/Game/VirtualRealityBP/Blueprints/BP_MotionController.LaserStaticMesh` (`/Game/VirtualRealityBP/Blueprints/MotionControllerPawn.RightController` _asmotion_controller_pawn)) false true)
  (`SceneComponent.SetVisibility` (`/Game/VirtualRealityBP/Blueprints/BP_MotionController.LaserStaticMesh` (`/Game/VirtualRealityBP/Blueprints/MotionControllerPawn.LeftController` _asmotion_controller_pawn)) false true))

(event `self.ReceiveTick`
  (params (DeltaSeconds :type "Float (single-precision)"))
  (add `/Game/Project/Blueprints/Points/MC/MC_Accident6.YouWon` (`self.Accident6`) (delegate `YouWon`))
  (add `/Game/Project/Blueprints/BP_Shinigami.GameOver` (`self.Shinigami`) (delegate `OnGameOver`)))

(event `YouWon`
  (bind _asmotion_controller_pawn (cast `/Game/VirtualRealityBP/Blueprints/MotionControllerPawn` (`GameplayStatics.GetPlayerPawn` 0) :!label _label))
  (`SceneComponent.SetVisibility` (`/Game/VirtualRealityBP/Blueprints/BP_MotionController.LaserStaticMesh` (`/Game/VirtualRealityBP/Blueprints/MotionControllerPawn.RightController` _asmotion_controller_pawn)) true true)
  (`SceneComponent.SetVisibility` (`/Game/VirtualRealityBP/Blueprints/BP_MotionController.LaserStaticMesh` (`/Game/VirtualRealityBP/Blueprints/MotionControllerPawn.LeftController` _asmotion_controller_pawn)) true true))

(event `OnGameOver`
  (goto _label))

(fn `UserConstructionScript`)