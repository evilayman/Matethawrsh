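; Endless-mode character that walks a list of points and collects safety gear: helmet, eyewear and gloves.
; Gear pickups that hit its capsule are destroyed and revealed on the PoseableMesh by toggling material sections.
; The W_Charachter widget shows icons for gear still missing, with state based on the current point.
; Each finished point advances movement and asks CharacterGenerator to spawn; reaching EP_Exit decrements its count and destroys the character after a delay.
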(event `self.ReceiveBeginPlay`
  (set `self.SpawnTime` (`GameplayStatics.GetRealTimeSeconds`))
  (`self.ToggleHat` (`self.isWearHat`))
  (`self.ToggleEyeWear` (`self.IsWearEyeWear`))
  (`self.ToggleGloves` (`self.IsWearGloves`))
  (`parent.ReceiveBeginPlay`)
  (`self.GetUIItems` (`self.Points`)))

(event `self.CapsuleComponent.OnComponentHit`
  (params (HitComponent :type "PrimitiveComponent Object Reference") (OtherActor :type "Actor Object Reference") (OtherComp :type "PrimitiveComponent Object Reference") (NormalImpulse :type "Vector Structure") (Hit :type "HitResult Structure (by ref)"))
  (`self.CheckOverlap` OtherActor)
  (`self.GetUIItems` (`self.Points`)))

(event `PointDone`
  (bind _output (`|GetArrayItem` (`self.Points`) (`self.CurrentIndex`)))
  ;[1 1 1] OnPointDone
  (`/Engine/EditorBlueprintResources/StandardMacros.IncrementInt` (`self.CurrentIndex`)
    (:`  `
      (`self.GetUIItems` (`self.Points`))
      (set `self.NextPoint` _output)
      (`self.MoveToPoint` _output)
      (`/Game/Project/Blueprints/EndlessMode/CharacterGenerator.TryGenerate` (`self.CharacterGenerator`))
      (cast `/Game/Project/Blueprints/EndlessMode/EP_Exit` _output)
      (`self.AllPointsDone`))))

(event `AllPointsDone`
  ;[1 1 1] All Points Done
  (`/Engine/EditorBlueprintResources/StandardMacros.DecrementInt` (`/Game/Project/Blueprints/EndlessMode/CharacterGenerator.CharactersCount` (`self.CharacterGenerator`))
    (:`  `
      (`KismetSystemLibrary.Delay` 10.0)
      (`self.K2_DestroyActor`))))

(fn `CheckOverlap`
  (params (Actor :type "Actor Object Reference"))
  (bind _asbp_hemlt_hats (cast `/Game/Project/Blueprints/SafetyEquipments/BP_hemlt_Hats` Actor)
    (:`then`
      (`self.ToggleHat` true)
      (`self.K2_DestroyActor` _asbp_hemlt_hats))
    (:`CastFailed`
      (bind _asbp_eyewear (cast `/Game/Project/Blueprints/SafetyEquipments/BP_EYEWEAR` Actor)
        (:`then`
          (`self.ToggleEyeWear` true)
          (`self.K2_DestroyActor` _asbp_eyewear))
        (:`CastFailed`
          (bind _asbp_gloves_gloves_2 (cast `/Game/Project/Blueprints/SafetyEquipments/BP_GLOVES_gloves_2` Actor))
          (`self.ToggleGloves` true)
          (`self.K2_DestroyActor` _asbp_gloves_gloves_2))))))

(fn `GetCurrentPointTime`
  (returns (Time :type "Float (double-precision)"))
  (if (< (`self.CurrentIndex`) (`KismetArrayLibrary.Array_Length` (`self.PointsTimes`)))
    (return (`|GetArrayItem` (`self.PointsTimes`) (`self.CurrentIndex`)))
    (else
      (return 0.0))))

(fn `GetUIItems`
  (params (Points :type "Array of /Game/Project/Blueprints/Points/BP_Point Object Reference"))
  (locals (W_character :type "/Game/Project/Widgets/Character/W_Charachter Object Reference"))
  (bind _asw_charachter (cast `/Game/Project/Widgets/Character/W_Charachter` (`WidgetComponent.GetUserWidgetObject` (`self.Widget`))))
  (set `local.W_character` _asw_charachter)
  (for (_array_element _array_index) Points
    (switch `/Game/Project/Blueprints/EndlessMode/SafetyType` (`/Game/Project/Blueprints/Points/BP_Point.PointType` _array_element)
      (:`NewEnumerator0`
        (bind _tooluistate (`self.GetUIItemState` _array_index))
        (bind _visibility (`self.GetUIItemVisiblity` (`self.IsWearGloves`)))
        (`/Game/Project/Widgets/Character/W_Charachter.SetGlovesEnable` (`local.W_character`) _tooluistate _visibility))
      (:`NewEnumerator1`
        (bind _tooluistate_2 (`self.GetUIItemState` _array_index))
        (bind _visibility_2 (`self.GetUIItemVisiblity` (`self.isWearHat`)))
        (`/Game/Project/Widgets/Character/W_Charachter.SetHelmetEnable` (`local.W_character`) _tooluistate_2 _visibility_2))
      (:`NewEnumerator2`
        (bind _tooluistate_3 (`self.GetUIItemState` _array_index))
        (bind _visibility_3 (`self.GetUIItemVisiblity` (`self.IsWearEyeWear`)))
        (`/Game/Project/Widgets/Character/W_Charachter.SetEyeWearEnable` (`local.W_character`) _tooluistate_3 _visibility_3))))
  (`/Game/Project/Widgets/Character/W_Charachter.RearrangeIcons` (`local.W_character`) Points))

(fn `GetUIItemState`
  (params (Index :type Integer))
  (returns (ToolUIState :type "/Game/Project/Widgets/Character/ToolsUIState Enum"))
  (if (== (`self.CurrentIndex`) Index)
    (return "NewEnumerator0")
    (else
      (return "NewEnumerator1"))))

(fn `GetUIItemVisiblity`
  (params (IsWear :type Boolean))
  (returns (Visibility :type "ESlateVisibility Enum"))
  (if IsWear
    (return "Collapsed")
    (else
      (return "Visible"))))

(fn `SetAliveTime`
  (bind _output_get (set `self.AliveTime` (- (`GameplayStatics.GetRealTimeSeconds`) (`self.SpawnTime`))))
  (`KismetSystemLibrary.PrintString` (`KismetStringLibrary.Conv_DoubleToString` _output_get) true true (struct :`G` 0.66 :`B` 1.0 :`A` 1.0) 10.0))

(fn `ToggleEyeWear`
  (params (Visibilty :type Boolean))
  (`SkinnedMeshComponent.ShowMaterialSection` (`self.PoseableMesh`) (`self.M_EyeWear_ID`) Visibilty 0)
  (set `self.IsWearEyeWear` Visibilty))

(fn `ToggleGloves`
  (params (Visibilty :type Boolean))
  (`SkinnedMeshComponent.ShowMaterialSection` (`self.PoseableMesh`) (`self.M_Gloves_ID`) Visibilty 0)
  (set `self.IsWearGloves` Visibilty))

(fn `ToggleHat`
  (params (Visibilty :type Boolean))
  (`SkinnedMeshComponent.ShowMaterialSection` (`self.PoseableMesh`) (`self.M_Hat_ID`) Visibilty 0)
  (set `self.isWearHat` Visibilty))

(fn `UserConstructionScript`
  (`parent.UserConstructionScript`))