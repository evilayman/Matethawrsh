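; BP_MC is a character that puts on safety gear (vest, hard hat, eyewear, gloves) when its capsule hits the matching item.
; Capsule hits go to IsOverlabWithSaftyTool, which identifies the item through a chain of casts and calls WearSafetyTool.
; WearSafetyTool shows or hides that gear's material section on the poseable mesh and updates its by-ref worn flag.
; DisableAllSafetyTools hides all four pieces, but its call in the event graph is unconnected.
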(event `self.ReceiveBeginPlay`
  (`parent.ReceiveBeginPlay`))

(event `self.ReceiveActorBeginOverlap`
  (params (OtherActor :type "Actor Object Reference"))
  (`parent.ReceiveActorBeginOverlap` OtherActor))

(event `self.CapsuleComponent.OnComponentHit`
  (params (HitComponent :type "PrimitiveComponent Object Reference") (OtherActor :type "Actor Object Reference") (OtherComp :type "PrimitiveComponent Object Reference") (NormalImpulse :type "Vector Structure") (Hit :type "HitResult Structure (by ref)"))
  (`self.IsOverlabWithSaftyTool` OtherActor))

(fn `DisableAllSafetyTools`
  (`self.WearSafetyTool` (`self.M_Vest_ID`) (`self.IsWearVest`))
  (`self.WearSafetyTool` (`self.M_Hat_ID`) (`self.IsWearHat`))
  (`self.WearSafetyTool` (`self.M_EyeWear_ID`) (`self.IsWearEyeWear`))
  (`self.WearSafetyTool` (`self.M_Gloves_ID`) (`self.IsWearGloves`)))

(fn `IsOverlabWithSaftyTool`
  (params (Actor :type "Actor Object Reference"))
  (cast `/Game/Project/Blueprints/SafetyEquipments/BP_vest` Actor
    (:`then`
      (`self.WearSafetyTool` (`self.M_Vest_ID`) (`self.IsWearVest`) true))
    (:`CastFailed`
      (cast `/Game/Project/Blueprints/SafetyEquipments/BP_hemlt_Hats` Actor
        (:`then`
          (`self.WearSafetyTool` (`self.M_Hat_ID`) (`self.IsWearHat`) true))
        (:`CastFailed`
          (cast `/Game/Project/Blueprints/SafetyEquipments/BP_EYEWEAR` Actor
            (:`then`
              (`self.WearSafetyTool` (`self.M_EyeWear_ID`) (`self.IsWearEyeWear`) true))
            (:`CastFailed`
              (cast `/Game/Project/Blueprints/SafetyEquipments/BP_GLOVES_gloves_2` Actor)
              (`self.WearSafetyTool` (`self.M_Gloves_ID`) (`self.IsWearGloves`) true))))))))

(fn `UserConstructionScript`
  (`parent.UserConstructionScript`))

(fn `WearSafetyTool`
  (params (MaterialID :type Integer) (IsWear :type "Boolean (by ref)") (Show :type Boolean))
  (`SkinnedMeshComponent.ShowMaterialSection` (`self.PoseableMesh`) MaterialID Show 0)
  (`|VariableSetRef` IsWear Show))