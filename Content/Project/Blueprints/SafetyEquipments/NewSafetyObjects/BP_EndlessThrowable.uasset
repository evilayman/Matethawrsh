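; BP_EndlessThrowable is a throwable object for the endless game, with a mesh and a toggleable trail effect.
; Hitting a BP_EndlessCharacter calls that character's CheckItemOverlap, while hits against other throwables are ignored.
; All other hits, including character hits, set IsHit after a short delay, then destroy the actor after a longer one unless DestroyCheck is set.
; ToggleTrail activates or deactivates the trail.
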(event `self.EndlessMesh.OnComponentHit`
  (params (HitComponent :type "PrimitiveComponent Object Reference") (OtherActor :type "Actor Object Reference") (OtherComp :type "PrimitiveComponent Object Reference") (NormalImpulse :type "Vector Structure") (Hit :type "HitResult Structure (by ref)"))
  (bind _asbp_endless_character (cast `/Game/Project/Blueprints/EndlessMode/BP_EndlessCharacter` OtherActor)
    (:`then`
      (`/Game/Project/Blueprints/EndlessMode/BP_EndlessCharacter.CheckItemOverlap` _asbp_endless_character self))
    (:`CastFailed`
      (cast `/Game/Project/Blueprints/SafetyEquipments/NewSafetyObjects/BP_EndlessThrowable` OtherActor
        (:`CastFailed`
          _))))
  (`KismetSystemLibrary.Delay` 1.0)
  (set `self.isHit` true)
  (`KismetSystemLibrary.Delay` 5.0)
  (if (not (`self.DestroyCheck`))
    (`self.K2_DestroyActor`)))

(fn `ToggleTrail`
  (params (Visisble :type Boolean))
  (bind _trail (`self.Trail`))
  (if Visisble
    (`ActorComponent.Activate` _trail true)
    (else
      (`ActorComponent.Deactivate` _trail))))

(fn `UserConstructionScript`)