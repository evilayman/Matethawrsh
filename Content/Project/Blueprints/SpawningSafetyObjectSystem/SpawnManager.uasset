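; Spawn manager that launches safety objects from a pool of spawn points toward the player controller's location.
; SpawnObject picks a random unused point (only indices 0–2 are handled), spawns the given class and applies a random-strength force with random positive Y/Z deviation.
; It removes and returns the used point; ReturnSafetyObjectToUnusedList adds its argument back to the pool, which BeginPlay fills from SpawnPointList.
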(event `self.ReceiveBeginPlay`
  (set `self.spawnPointUnusedList` (`self.spawnPointList`))
  (set `self.player` (`GameplayStatics.GetPlayerController` 0)))

(fn `ReturnSafetyObjectToUnusedList`
  (params (safetyObject :type "/Game/Project/Blueprints/SpawningSafetyObjectSystem/SpawnPointBP Object Reference"))
  (`KismetArrayLibrary.Array_Add` (`self.spawnPointUnusedList`) safetyObject))

(fn `SpawnObject`
  (params (SafetyObject :type "/Game/Project/Blueprints/BP_Rewind/BP_RewindableObject Class Reference"))
  (returns (spawnedSafetyObject :type "/Game/Project/Blueprints/SpawningSafetyObjectSystem/SpawnPointBP Object Reference"))
  (locals (tempSpawnPoint :type "/Game/Project/Blueprints/SpawningSafetyObjectSystem/SpawnPointBP Object Reference"))
  (bind _returnvalue (`KismetMathLibrary.RandomFloatInRange` 0.0 (`self.deviationRange`)))
  (bind _output (`|GetArrayItem` (`self.spawnPointUnusedList`) (`self.randomNumber`)))
  (bind (_returnvalue_x _returnvalue_y _returnvalue_z) (`KismetMathLibrary.BreakVector` (`KismetMathLibrary.GetDirectionUnitVector` (`self.K2_GetActorLocation` (`self.spawnPoint`)) (`self.K2_GetActorLocation` (`self.player`)))))
  (bind _output_get (set `self.randomNumber` (`KismetMathLibrary.RandomInteger` (`KismetArrayLibrary.Array_Length` (`self.spawnPointUnusedList`)))))
  (switch `int` _output_get
    (:`0`
      _)
    (:`1`
      _)
    (:`2`
      _))
  (`/Engine/EditorBlueprintResources/StandardMacros.IsValid` _output
    (:`Is Valid`
      (bind _output_get_2 (set `self.spawnPoint` _output))
      (bind _returnvalue_2 (`|SpawnActorFromClass` SafetyObject (`self.GetTransform` _output_get_2) "AdjustIfPossibleButAlwaysSpawn" "OverrideRootScale" null null))
      (`PrimitiveComponent.AddForce` (`StaticMeshActor.StaticMeshComponent` _returnvalue_2) (* (`KismetMathLibrary.MakeVector` _returnvalue_x (+ _returnvalue_y _returnvalue) (+ _returnvalue_z _returnvalue)) (`KismetMathLibrary.RandomFloatInRange` (`self.minForce`) (`self.maxForce`))) "None" false)
      (bind _output_get_3 (set `local.tempSpawnPoint` (`|GetArrayItem` (`self.spawnPointUnusedList`) (`self.randomNumber`))))
      (`KismetArrayLibrary.Array_Remove` (`self.spawnPointUnusedList`) (`self.randomNumber`))
      (return _output_get_3))))

(fn `UserConstructionScript`)