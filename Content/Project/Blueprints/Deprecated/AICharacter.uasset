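; Deprecated AI character that runs a behavior tree to move between an array of Target actors and can be paused while its rewind component is active.
; Tick pushes the current target and a Pause flag, driven by the rewindable animated component, to the blackboard.
; Capsule overlaps trigger each Target's action and leave action and toggle Arrived and Moving, while ChangeTarget cycles the index with wraparound.
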(event `self.ReceiveBeginPlay`
  (set `self.CurrentTarget` (`|GetArrayItem` (`self.Targets`) (`self.CurrentTargetIndex`)))
  (`AIController.RunBehaviorTree` (`AIBlueprintHelperLibrary.GetAIController` self) "/Game/Project/Blueprints/Deprecated/AI_BT.AI_BT")
  (`BlackboardComponent.SetValueAsObject` (`AIBlueprintHelperLibrary.GetBlackboard` self) "Target" (`self.CurrentTarget`)))

(event `self.ReceiveTick`
  (params (DeltaSeconds :type "Float (single-precision)"))
  (bind _returnvalue (== (`BlackboardComponent.GetValueAsInt` (`AIBlueprintHelperLibrary.GetBlackboard` self) "Pause") (`self.BTPause`)))
  (`BlackboardComponent.SetValueAsObject` (`AIBlueprintHelperLibrary.GetBlackboard` self) "Target" (`self.CurrentTarget`))
  (if (`/Game/Project/Blueprints/BP_Rewind/RewindableAnimatedComponent.RewindStarted` (`self.RewindableAnimatedComponent`))
    (set `self.BTPause` 1)
    (if (not _returnvalue)
      (`BlackboardComponent.SetValueAsInt` (`AIBlueprintHelperLibrary.GetBlackboard` self) "Pause" (`self.BTPause`) :!label _label))
    (else
      (set `self.BTPause` 0)
      (if (not _returnvalue)
        (goto _label)))))

(event `self.CapsuleComponent.OnComponentBeginOverlap`
  (params (OverlappedComponent :type "PrimitiveComponent Object Reference") (OtherActor :type "Actor Object Reference") (OtherComp :type "PrimitiveComponent Object Reference") (OtherBodyIndex :type Integer) (bFromSweep :type Boolean) (SweepResult :type "HitResult Structure (by ref)"))
  (bind _astarget (cast `/Game/Project/Blueprints/Deprecated/Targets/Target` OtherActor))
  (`/Game/Project/Blueprints/Deprecated/Targets/Target.DoAction` _astarget self (`self.RewindableAnimatedComponent`))
  (set `self.Arrived` true)
  (set `self.Moving` false))

(event `self.CapsuleComponent.OnComponentEndOverlap`
  (params (OverlappedComponent :type "PrimitiveComponent Object Reference") (OtherActor :type "Actor Object Reference") (OtherComp :type "PrimitiveComponent Object Reference") (OtherBodyIndex :type Integer))
  (bind _astarget (cast `/Game/Project/Blueprints/Deprecated/Targets/Target` OtherActor))
  (`/Game/Project/Blueprints/Deprecated/Targets/Target.DoLeaveAction` _astarget)
  (set `self.Arrived` false)
  (set `self.Moving` true))

(event `ChangeTarget`
  (bind _result (`/Engine/EditorBlueprintResources/StandardMacros.IncrementInt` (`self.CurrentTargetIndex`))
    (:`  `
      (if (>= _result (`KismetArrayLibrary.Array_Length` (`self.Targets`)))
        (set `self.CurrentTargetIndex` 0)
        (set `self.CurrentTarget` (`|GetArrayItem` (`self.Targets`) (`self.CurrentTargetIndex`)))
        (else
          (set `self.CurrentTarget` (`|GetArrayItem` (`self.Targets`) (`self.CurrentTargetIndex`))))))))

(fn `UserConstructionScript`)