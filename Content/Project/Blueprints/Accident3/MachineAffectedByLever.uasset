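; Machine actor that rotates in response to a lever's Up or Down movement and tracks a DoorOpened flag.
; LeverMoved plays or reverses the RotateMachineUp timeline, whose update sets roll from its angle curve scaled by TargetRotation, zeroing pitch and yaw.
; A separate RotateTheMachine function, not called within this Blueprint, instead interpolates yaw per call using RInterpTo and RotationSpeed, gated by angle limits.
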(event `self.ReceiveBeginPlay`
  (set `self.DoorOpened` false))

(event `/Game/Project/Blueprints/Accident3/iLeverMoved.LeverMoved`
  (params (Direction :type String))
  (switch `string` Direction
    (:`Up`
      (set `self.DoorOpened` true)
      (bind (_direction _angle) (`Timeline|RotateMachineUp` :!label _label)
        (:`Update`
          (`self.K2_SetActorRotation` (`KismetMathLibrary.MakeRotator` (* (.z _angle) (`self.TargetRotation`)))))))
    (:`Down`
      (set `self.DoorOpened` false)
      (goto _label :!via `Reverse`))))

(fn `RotateTheMachine`
  (params (Direction :type String))
  (switch `string` Direction
    (:`Up`
      (if (<= (.yaw (`self.K2_GetActorRotation`)) 45.0)
        (`self.K2_SetActorRotation` (`KismetMathLibrary.RInterpTo` (`self.K2_GetActorRotation`) (`KismetMathLibrary.MakeRotator` 0.0 0.0 (`KismetMathLibrary.Abs` (`self.TargetRotation`))) (`GameplayStatics.GetWorldDeltaSeconds`) (`self.RotationSpeed`)))))
    (:`Down`
      (if (>= (.yaw (`self.K2_GetActorRotation`)) -45.0)
        (`self.K2_SetActorRotation` (`KismetMathLibrary.RInterpTo` (`self.K2_GetActorRotation`) (`KismetMathLibrary.MakeRotator` 0.0 0.0 (`self.TargetRotation`)) (`GameplayStatics.GetWorldDeltaSeconds`) (`self.RotationSpeed`)))))))

(fn `UserConstructionScript`)