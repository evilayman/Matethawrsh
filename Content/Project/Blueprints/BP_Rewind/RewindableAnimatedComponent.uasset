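; Actor component that records an animated physics actor's movement and skeleton pose, then plays it back in reverse.
; Tick appends transform, velocities, socket transforms and step timing to Record, capping repeated idle transform and velocity samples.
; StartRewind prunes the record through SkipRecord; Tick then pops samples from the end, passing bone poses to SkeletonController.
; An empty record triggers StopRewind, which fires a completion dispatcher and clears all buffers.
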(event `self.ReceiveBeginPlay`)

(event `self.ReceiveTick`
  (params (DeltaSeconds :type "Float (single-precision)"))
  (if (`self.RewindStarted`)
    (if (< (`KismetArrayLibrary.Array_LastIndex` (`.Transforms_3_920AE801440DC98B056C4D9D987D380F` (break `/Game/Project/Blueprints/BP_Rewind/RecordData` (`self.Record`)))) 0)
      (`self.StopRewind`)
      (else
        (`self.RewindOneStep` 0.0)))
    (elif (`self.RecordStarted`)
      (`self.RecordMovement`))))

(event `self.StartRecording`
  (params (MaxRedundantMoves :type Integer) (Record :type "/Game/Project/Blueprints/BP_Rewind/RecordData Structure (by ref)"))
  (set `self.Record` Record)
  (`self.StopRecording`)
  (`self.StopRewind`)
  (set `self.MaxRedundantMoves` MaxRedundantMoves)
  (set `self.RecordStarted` true))

(event `self.StopRecording`
  (set `self.RecordStarted` false))

(event `self.StartRewind`
  (params (Time :type "Float (single-precision)"))
  (`self.SkipRecord` 1)
  (`self.StopRecording`)
  (if (> (`KismetArrayLibrary.Array_Length` (`.Transforms_3_920AE801440DC98B056C4D9D987D380F` (break `/Game/Project/Blueprints/BP_Rewind/RecordData` (`self.Record`)))) 0)
    (if (not (`self.RewindStarted`))
      (set `SkeletonController.RewindStarted` true (`Actor.GetComponentByClass` (`self.GetOwner`) "/Script/Matethawrsh.SkeletonController"))
      (set `self.RewindStarted` true))))

(event `self.StopRewind`
  (bind (_transforms _linearvels _angularvels _bonedata _stepdurations) (break `/Game/Project/Blueprints/BP_Rewind/RecordData` (`self.Record`)))
  (if (`self.RewindStarted`)
    (`self.Disp_RewindCompleted`))
  (set `SkeletonController.RewindStarted` false (`Actor.GetComponentByClass` (`self.GetOwner`) "/Script/Matethawrsh.SkeletonController"))
  (set `self.RewindStarted` false)
  (set `self.IsRewinding` false)
  (`KismetArrayLibrary.Array_Clear` _transforms)
  (`KismetArrayLibrary.Array_Clear` _linearvels)
  (`KismetArrayLibrary.Array_Clear` _angularvels)
  (`KismetArrayLibrary.Array_Clear` _bonedata)
  (set `self.RedundantMovesCounter` 0)
  (`KismetArrayLibrary.Array_Clear` _stepdurations))

(fn `RecordMovement`
  (locals (BoneTransforms :type "Array of Transform Structure") (StepTime :type "Float (double-precision)"))
  (bind _returnvalue (`self.GetOwner`))
  (bind _returnvalue_2 (`self.GetOwner`))
  (bind (_transforms _linearvels _angularvels _bonedata _stepdurations) (break `/Game/Project/Blueprints/BP_Rewind/RecordData` (`self.Record`)))
  (bind (_transforms_2 _linearvels_2 _angularvels_2 _bonedata_2) (break `/Game/Project/Blueprints/BP_Rewind/RecordData` (`self.Record`)))
  (bind _returnvalue_3 (`Actor.GetComponentByClass` _returnvalue "/Script/Engine.PrimitiveComponent"))
  (bind _returnvalue_4 (`Actor.GetComponentByClass` (`self.GetOwner`) "/Script/Engine.SkeletalMeshComponent"))
  (bind _returnvalue_5 (`Actor.GetComponentByClass` _returnvalue_2 "/Script/Engine.PrimitiveComponent"))
  (bind _returnvalue_6 (`PrimitiveComponent.GetPhysicsAngularVelocityInDegrees` _returnvalue_5 "None"))
  (set `local.StepTime` (`.PartialSeconds` (`GameplayStatics.GetAccurateRealTime`)))
  (if (> (`KismetArrayLibrary.Array_Length` _transforms) 0)
    (`|ExecutionSequence`
      (:`then_0`
        (if (== (`|GetArrayItem` _transforms_2 (`KismetArrayLibrary.Array_LastIndex` _transforms_2)) (`Actor.GetTransform` _returnvalue_2))
          (bind _result (`/Engine/EditorBlueprintResources/StandardMacros.IncrementInt` (`self.RedundantMovesCounter`))
            (:`  `
              (if (not (>= _result (`self.MaxRedundantMoves`)))
                (`KismetArrayLibrary.Array_Add` _transforms_2 (`Actor.GetTransform` _returnvalue_2) :!label _label))))
          (else
            (set `self.RedundantMovesCounter` 0)
            (goto _label))))
      (:`then_1`
        (bind _returnvalue_7 (`PrimitiveComponent.GetPhysicsLinearVelocity` _returnvalue_5 "None"))
        (if (== (`|GetArrayItem` _linearvels_2 (`KismetArrayLibrary.Array_LastIndex` _linearvels_2)) _returnvalue_7)
          (if (not (>= (`self.RedundantMovesCounter`) (`self.MaxRedundantMoves`)))
            (`KismetArrayLibrary.Array_Add` _linearvels_2 _returnvalue_7 :!label _label_2))
          (else
            (goto _label_2))))
      (:`then_2`
        (if (== (`|GetArrayItem` _angularvels_2 (`KismetArrayLibrary.Array_LastIndex` _angularvels_2)) _returnvalue_6)
          (if (not (>= (`self.RedundantMovesCounter`) (`self.MaxRedundantMoves`)))
            (`KismetArrayLibrary.Array_Add` _angularvels_2 _returnvalue_6 :!label _label_3))
          (else
            (goto _label_3))))
      (:`then_3`
        (if (>= (`self.RedundantMovesCounter`) (`self.MaxRedundantMoves`)) :!label _label_4
          _
          (else
            _))
        (for _array_element (`SceneComponent.GetAllSocketNames` _returnvalue_4)
          (`KismetArrayLibrary.Array_Add` (`local.BoneTransforms`) (`SceneComponent.GetSocketTransform` _returnvalue_4 _array_element "RTS_World")))
        (`KismetArrayLibrary.Array_Add` _bonedata_2 (make `/Game/Project/Blueprints/BP_Rewind/SkeletonBoneTransforms` (`local.BoneTransforms`))))
      (:`then_4`
        (bind _output_get (set `local.StepTime` (- (`.PartialSeconds` (`GameplayStatics.GetAccurateRealTime`)) (`local.StepTime`))))
        (`KismetArrayLibrary.Array_Add` (`.StepDurations_12_9278CDB94170104F3786E6BC343F7247` (break `/Game/Project/Blueprints/BP_Rewind/RecordData` (`self.Record`))) _output_get)))
    (else
      (`KismetArrayLibrary.Array_Add` _stepdurations)
      (`KismetArrayLibrary.Array_Add` _transforms (`Actor.GetTransform` _returnvalue))
      (bind _returnvalue_8 (`PrimitiveComponent.GetPhysicsLinearVelocity` _returnvalue_3 "None"))
      (`KismetArrayLibrary.Array_Add` _linearvels _returnvalue_8)
      (`KismetArrayLibrary.Array_Add` _angularvels (`PrimitiveComponent.GetPhysicsAngularVelocityInDegrees` _returnvalue_3 "None"))
      (goto _label_4))))

(fn `SkipRecord`
  (params (SkipRate :type Integer))
  (bind (_transforms _linearvels _angularvels _bonedata _stepdurations) (break `/Game/Project/Blueprints/BP_Rewind/RecordData` (`self.Record`)))
  (if (!= SkipRate 0)
    (for _index (range (+ (`KismetArrayLibrary.Array_Length` (`.Transforms_3_920AE801440DC98B056C4D9D987D380F` (break `/Game/Project/Blueprints/BP_Rewind/RecordData` (`self.Record`)))) 1))
      (if (== (mod _index SkipRate) 0)
        (`KismetArrayLibrary.Array_Remove` _transforms _index)
        (`KismetArrayLibrary.Array_Remove` _linearvels _index)
        (`KismetArrayLibrary.Array_Remove` _angularvels _index)
        (`KismetArrayLibrary.Array_Remove` _bonedata _index)
        (`KismetArrayLibrary.Array_Remove` _stepdurations _index)))))