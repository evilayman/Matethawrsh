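; Forklift actor that loops along a list of waypoints, returning to its start position before each repeat.
; Timelines alternate lerped moves with yaw turns toward the next point, consuming a working copy of OriginalPoints that is refilled when empty.
; Wheels spin forward during moves, and Tick spins them backward while the RewindableObjectComponent has rewind started.
; A separate MoveForkWithParam event lerps the forklift to a given position.
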(event `self.ReceiveBeginPlay`
  (`self.CopyPointsArray`)
  (`self.MoveFork`)
  (set `self.PointZero` (`self.K2_GetActorLocation`)))

(event `MoveFork`
  (bind _points (`self.Points`))
  (bind _points_2 (`self.Points`))
  (set `self.ForkStartPos` (`self.K2_GetActorLocation`))
  (if (> (`KismetArrayLibrary.Array_Length` _points_2) 0)
    (bind (_direction _alpha) (`Timeline|MoveForkLift` :!via `PlayFromStart` :!label _label)
      (:`Update`
        (`self.K2_SetActorLocation` (`KismetMathLibrary.VLerp` (`self.ForkStartPos`) (`|GetArrayItem` _points) _alpha))
        (`SceneComponent.K2_AddLocalRotation` (`self.RightWheel_Front`) (struct :`Roll` 5.0) false false)
        (`SceneComponent.K2_AddLocalRotation` (`self.LeftWheel_Back`) (struct :`Roll` 5.0) false false)
        (`SceneComponent.K2_AddLocalRotation` (`self.RightWheel_Back`) (struct :`Roll` 5.0) false false)
        (`SceneComponent.K2_AddLocalRotation` (`self.LeftWheel_Front`) (struct :`Roll` 5.0) false false))
      (:`Finished`
        (`KismetArrayLibrary.Array_Remove` _points)
        (if (> (`KismetArrayLibrary.Array_Length` (`self.Points`)) 0)
          (set `self.TargetRotation` (`|GetArrayItem` (`self.Points`)))
          (bind (_direction_2 _angle) (`Timeline|RotateForkLift` :!via `PlayFromStart` :!label _label_2)
            (:`Update`
              (bind (_returnvalue_roll _returnvalue_pitch _returnvalue_yaw) (`KismetMathLibrary.BreakRotator` (`KismetMathLibrary.RLerp` (`self.K2_GetActorRotation`) (`KismetMathLibrary.FindLookAtRotation` (`self.K2_GetActorLocation`) (`self.TargetRotation`)) _angle)))
              (`self.K2_SetActorRotation` (`KismetMathLibrary.MakeRotator` 0.0 0.0 _returnvalue_yaw)))
            (:`Finished`
              (`self.MoveFork`)))
          (else
            (set `self.TargetRotation` (`self.PointZero`))
            (goto _label_2 :!via `PlayFromStart`)))))
    (else
      (`KismetArrayLibrary.Array_Add` _points_2 (`self.PointZero`))
      (`self.CopyPointsArray`)
      (goto _label :!via `PlayFromStart`))))

(event `MoveForkWithParam`
  (params (NewPosition :type "Vector Structure"))
  (bind _output_get (set `self.ForkStartPosParam` (`self.K2_GetActorLocation`)))
  (bind (_direction _alpha) (`Timeline|MoveForkToPos`)
    (:`Update`
      (`self.K2_SetActorLocation` (`KismetMathLibrary.VLerp` _output_get NewPosition _alpha))
      (`SceneComponent.K2_AddLocalRotation` (`self.RightWheel_Front`) (struct :`Roll` 5.0) false false)
      (`SceneComponent.K2_AddLocalRotation` (`self.LeftWheel_Back`) (struct :`Roll` 5.0) false false)
      (`SceneComponent.K2_AddLocalRotation` (`self.RightWheel_Back`) (struct :`Roll` 5.0) false false)
      (`SceneComponent.K2_AddLocalRotation` (`self.LeftWheel_Front`) (struct :`Roll` 5.0) false false))))

(event `self.ReceiveTick`
  (params (DeltaSeconds :type "Float (single-precision)"))
  (`parent.ReceiveTick` DeltaSeconds)
  (if (`/Game/Project/Blueprints/BP_Rewind/RewindableObjectComponent.RewindStarted` (`self.RewindableObjectComponent`))
    (`SceneComponent.K2_AddLocalRotation` (`self.RightWheel_Front`) (struct :`Roll` -5.0) false false)
    (`SceneComponent.K2_AddLocalRotation` (`self.LeftWheel_Back`) (struct :`Roll` -5.0) false false)
    (`SceneComponent.K2_AddLocalRotation` (`self.RightWheel_Back`) (struct :`Roll` -5.0) false false)
    (`SceneComponent.K2_AddLocalRotation` (`self.LeftWheel_Front`) (struct :`Roll` -5.0) false false)))

(fn `CopyPointsArray`
  (for _array_element (`self.OriginalPoints`)
    (`KismetArrayLibrary.Array_Add` (`self.Points`) _array_element)))

(fn `UserConstructionScript`)