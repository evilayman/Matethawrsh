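; EP_Hat is an Endless Mode point Blueprint that handles a character arriving at a hat point.
; Forward and rewind arrivals call their parent events, then share one path that sets the active state and waits for the character's current point time.
; It then marks the work done, and deactivates and completes the point only if the character is wearing a hat.
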(event `self.OnPointArrive`
  (params (RewindableCharacter :type "/Game/Project/Blueprints/BP_Rewind/BP_RewindableCharacter Object Reference"))
  (`parent.OnPointArrive` RewindableCharacter)
  (`self.SetActiveState` (`self.ActiveState`) :!label _label)
  (bind _time (`/Game/Project/Blueprints/EndlessMode/BP_EndlessCharacter.GetCurrentPointTime` (`self.EndlessCharacter`)))
  (`KismetSystemLibrary.Delay` _time)
  (`self.SetWorkDone` true)
  (if (`/Game/Project/Blueprints/EndlessMode/BP_EndlessCharacter.isWearHat` (`self.EndlessCharacter`))
    (set `self.IsActive` false)
    (`self.PointDone`)))

(event `self.OnPointArriveRewind`
  (params (`Rewindable Character` :type "/Game/Project/Blueprints/BP_Rewind/BP_RewindableCharacter Object Reference"))
  (`parent.OnPointArriveRewind` `Rewindable Character`)
  (goto _label))

(fn `UserConstructionScript`
  (`parent.UserConstructionScript`))