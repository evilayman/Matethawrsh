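; AI-driven character that moves between point actors, can ragdoll, and recovers when its RewindableAnimatedComponent finishes a rewind.
; It displays a PoseableMesh over a hidden skeletal Mesh; rewind completion snaps the Mesh to it, clears physics and resumes movement.
; Arrivals notify the point, with a separate callback after rewind.
; Callable events drive speech, focus, look-at, animation state, object pickup/drop and panic movement that suspends point-to-point moves.
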(event `self.ReceiveBeginPlay`
  ;[1 1 1] Init Visibilty, Bind to Dispatcher and Start Moving
  (`SceneComponent.SetVisibility` (`self.Mesh`) false true)
  (`SceneComponent.SetVisibility` (`self.PoseableMesh`) true true)
  (add `/Game/Project/Blueprints/BP_Rewind/RewindableAnimatedComponent.Disp_RewindCompleted` (`self.RewindableAnimatedComponent`) (delegate `OnRewindCompleted`)))

(event `OnRewindCompleted`
  ;[1 1 1] Init Visibilty, Bind to Dispatcher and Start Moving
  (set `self.RewindComplete` true)
  (`self.Reset Character`))

(event `Reset Character`
  (bind _mesh (`self.Mesh`))
  ;[1 1 1] Reset Character
  (set `self.InPanic` false)
  (`AIController.K2_ClearFocus` (`AIBlueprintHelperLibrary.GetAIController` self))
  (`self.SetActiveState` 0)
  (`SkeletalMeshComponent.SetAnimationMode` (`self.Mesh`) "AnimationBlueprint")
  (`SkeletalMeshComponent.K2_SetAnimInstanceClass` (`self.Mesh`) "/Game/Project/MainCharacter/AnimationBP_MC.AnimationBP_MC_C")
  (`ActorComponent.Deactivate` (`self.PoseableMesh`))
  (`SceneComponent.K2_AttachToComponent` (`self.Mesh`) (`self.CapsuleComponent`) "None" "KeepRelative" "KeepRelative" "KeepRelative" true)
  (`SceneComponent.K2_SetWorldTransform` (`self.Mesh`) (`SceneComponent.K2_GetComponentToWorld` (`self.PoseableMesh`)) false true)
  (`PrimitiveComponent.SetCollisionEnabled` _mesh "QueryOnly")
  (`SkeletalMeshComponent.SetAllBodiesSimulatePhysics` _mesh false)
  (`SkeletalMeshComponent.SetAllBodiesPhysicsBlendWeight` _mesh 0.0 false)
  (`KismetSystemLibrary.Delay` 0.1)
  (`ActorComponent.Activate` (`self.PoseableMesh`) true)
  (`self.MoveToPoint` (`self.NextPoint`)))

(event `SimulateBones`
  (params (BlendWeight :type "Float (double-precision)"))
  (bind _mesh (`self.Mesh`))
  ;[1 1 1] Simulate Bones aka Death
  (`PrimitiveComponent.SetCollisionEnabled` _mesh "QueryAndPhysics")
  (`SkeletalMeshComponent.SetAllBodiesSimulatePhysics` _mesh true)
  (`SkeletalMeshComponent.SetAllBodiesPhysicsBlendWeight` _mesh BlendWeight false))

(event `MoveToPoint`
  (params (TargetPoint :type "/Game/Project/Blueprints/Points/BP_Point Object Reference") (Speed :type "Float (double-precision)" :default 150.0))
  (bind _nextpoint (`self.NextPoint`))
  ;[1 1 1] Move To Point
  (if (not (`self.InPanic`))
    (set `CharacterMovementComponent.MaxWalkSpeed` Speed (`self.CharacterMovement`))
    (bind _output_get (set `self.NextPoint` TargetPoint))
    (`|AIMoveTo` (`PawnMovementComponent.GetPawnOwner` (`self.CharacterMovement`)) (0.0 0.0 0.0) _output_get
      (:`OnSuccess`
        (if (`self.RewindComplete`)
          (`/Game/Project/Blueprints/Points/BP_Point.OnPointArriveRewind` _nextpoint self)
          (set `self.RewindComplete` false)
          (else
            (`/Game/Project/Blueprints/Points/BP_Point.OnPointArrive` _nextpoint self))))
      (:`OnFail`
        (`self.MoveToPoint` (`self.NextPoint`) Speed)))))

(event `TurnToLocation`
  (params (FocusPoint :type "Vector Structure") (BreakFocusEnabled :type Boolean :default true) (BreakFocusTime :type "Float (double-precision)"))
  (bind _returnvalue (`AIBlueprintHelperLibrary.GetAIController` self))
  ;[1 1 1] Turn to Location
  (`AIController.K2_SetFocalPoint` _returnvalue FocusPoint)
  (if BreakFocusEnabled
    (`KismetSystemLibrary.Delay` BreakFocusTime)
    (`AIController.K2_ClearFocus` _returnvalue)))

(event `TurnToActor`
  (params (TurnActor :type "Actor Object Reference") (BreakFocusEnabled :type Boolean :default true) (BreakFocusTime :type "Float (double-precision)"))
  (bind _returnvalue (`AIBlueprintHelperLibrary.GetAIController` self))
  ;[1 1 1] Turn to Actor
  (`AIController.K2_SetFocus` _returnvalue TurnActor)
  (if BreakFocusEnabled
    (`KismetSystemLibrary.Delay` BreakFocusTime)
    (`AIController.K2_ClearFocus` _returnvalue)))

(event `Speak`
  (params (Sound :type "SoundBase Object Reference"))
  ;[1 1 1] Speak
  (bind _returnvalue (`GameplayStatics.SpawnSoundAtLocation` Sound (`self.K2_GetActorLocation`) (struct) 1.0 1.0 0.0 "/Game/Project/Sounds/VoiceAttenuation.VoiceAttenuation" null))
  (set `self.SoundPlaying` _returnvalue))

(event `StopSpeak`
  (bind _soundplaying (`self.SoundPlaying`))
  ;[1 1 1] StopSpeak
  (`/Engine/EditorBlueprintResources/StandardMacros.IsValid` _soundplaying
    (:`Is Valid`
      (`AudioComponent.Stop` _soundplaying))))

(event `LookAtLocation`
  (params (LookLocation :type "Vector Structure") (LookDuration :type "Float (double-precision)"))
  ;[1 1 1] Look At Location
  (set `self.LookLocation` LookLocation)
  (set `self.LookEnabled` true)
  (`KismetSystemLibrary.Delay` LookDuration)
  (set `self.LookEnabled` false))

(event `LookAtActor`
  (params (`Look Actor` :type "Actor Object Reference") (`Look Duration` :type "Float (double-precision)"))
  ;[1 1 1] Look At Actor
  (set `self.LookActor` `Look Actor`)
  (set `self.LookEnabled` true)
  (`KismetSystemLibrary.Delay` `Look Duration`)
  (set `self.LookActor` null)
  (set `self.LookEnabled` false))

(event `self.ReceiveTick`
  (params (DeltaSeconds :type "Float (single-precision)"))
  ;[1 1 1] Tick Update
  (if (`KismetSystemLibrary.IsValid` (`self.LookActor`))
    (set `self.LookLocation` (`self.K2_GetActorLocation` (`self.LookActor`)))))

(event `SetActiveState`
  (params (ActiveState :type Integer))
  ;[1 1 1] Set AnimationBP Active State
  (set `self.ActiveState` ActiveState))

(event `SetWorkingDone`
  (params (isWorkingDone :type Boolean))
  ;[1 1 1] Set AnimationBP Working State
  (set `self.isWorkingDone` isWorkingDone))

(event `PickUpObject`
  (bind _targetobject (`self.TargetObject`))
  (bind _returnvalue (`self.GetComponentByClass` _targetobject "/Script/Engine.StaticMeshComponent"))
  ;[1 1 1] PickUp Object
  (if (not (`self.HoldingObject`))
    (set `self.HoldingObject` true)
    (`/Engine/EditorBlueprintResources/StandardMacros.IsValid` _targetobject
      (:`Is Valid`
        (`self.K2_AttachToComponent` _targetobject (`self.Mesh`) "LeftHandSocket" "SnapToTarget" "KeepRelative" "KeepWorld" true)
        (`PrimitiveComponent.SetSimulatePhysics` _returnvalue false)
        (`PrimitiveComponent.SetCollisionEnabled` _returnvalue "NoCollision")))
    (else
      (`self.DropObject`))))

(event `DropObject`
  (bind _targetobject (`self.TargetObject`))
  (bind _returnvalue (`self.GetComponentByClass` _targetobject "/Script/Engine.StaticMeshComponent"))
  ;[1 1 1] Drop Object
  (`/Engine/EditorBlueprintResources/StandardMacros.IsValid` _targetobject
    (:`Is Valid`
      (`self.K2_DetachFromActor` _targetobject "KeepWorld" "KeepWorld" "KeepWorld")
      (`PrimitiveComponent.SetSimulatePhysics` _returnvalue true)
      (`PrimitiveComponent.SetCollisionEnabled` _returnvalue "QueryAndPhysics")
      (set `self.TargetObject` null)
      (set `self.HoldingObject` false))))

(event `MoveToPanic`
  (params (Actor :type "Actor Object Reference") (Speed :type "Float (double-precision)" :default 400.0) (AcceptanceDistance :type "Float (double-precision)" :default 50.0))
  (bind _returnvalue (`self.K2_GetActorLocation` Actor))
  (bind _charactermovement (`self.CharacterMovement`))
  ;[1 1 1] Move To Actor Panic
  (set `CharacterMovementComponent.MaxWalkSpeed` Speed _charactermovement)
  (`self.SetActiveState` 7)
  (`|AIMoveTo` (`PawnMovementComponent.GetPawnOwner` _charactermovement) (+ (* (`KismetMathLibrary.GetDirectionUnitVector` _returnvalue (`self.K2_GetActorLocation`)) AcceptanceDistance) _returnvalue) null
    (:`then`
      (set `self.InPanic` true))))

(fn `UserConstructionScript`)