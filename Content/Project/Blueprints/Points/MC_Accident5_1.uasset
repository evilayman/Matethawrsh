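; Scripted path point for accident 5 that reacts when a rewindable character arrives, branching on whether the hole is safe.
; On arrival it turns the character, sets its active state and marks the work done.
; If MC.IsHoleSafe, it plays a speech line and routes to PNotFall; otherwise it routes to PFall, using timed delays before moving on.
; Arrival during rewind skips the sequence and just moves on.
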(event `self.OnPointArrive`
  (params (RewindableCharacter :type "/Game/Project/Blueprints/BP_Rewind/BP_RewindableCharacter Object Reference"))
  (`parent.OnPointArrive` RewindableCharacter)
  (`self.TurnToLocation` 1.0)
  (`self.SetActiveState` (`self.ActiveState`))
  (`self.SetWorkDone` true)
  (if (`/Game/Project/MainCharacter/BP_MC.IsHoleSafe` (`self.MC`))
    (`KismetSystemLibrary.Delay` 2.0)
    (`self.Speak` "NewEnumerator0" "/Game/Project/Sounds/MC_S2A2_Ha23FelMagary.MC_S2A2_Ha23FelMagary")
    (`KismetSystemLibrary.Delay` 3.1)
    (`self.SetActiveState` 0)
    (`KismetSystemLibrary.Delay` 0.5)
    (set `self.NextPoint` (`self.P_NotFall`))
    (`self.MoveOn` 150.0)
    (else
      (`KismetSystemLibrary.Delay` 2.0)
      (set `self.NextPoint` (`self.P_Fall`))
      (`self.SetActiveState` 0)
      (`self.MoveOn` 150.0))))

(event `self.OnPointArriveRewind`
  (params (`Rewindable Character` :type "/Game/Project/Blueprints/BP_Rewind/BP_RewindableCharacter Object Reference"))
  (`parent.OnPointArriveRewind` `Rewindable Character`)
  (`self.MoveOn` 150.0))

(fn `UserConstructionScript`
  (`parent.UserConstructionScript`))